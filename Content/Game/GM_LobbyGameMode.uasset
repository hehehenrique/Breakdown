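; GM_LobbyGameMode is the lobby game mode that places players at team-based spawn points.
; On BeginPlay it finds and caches the first BP_TDMSpawnManager in the level if none is set.
; RespawnPlayer reads the team from the player's PS_VehicleState, asks the spawn manager for an available spawn, and moves the player's existing actor to that point rather than spawning a new one.
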(event `self.ReceiveBeginPlay`
  (`/Engine/EditorBlueprintResources/StandardMacros.IsValid` (`self.TDM_SpawnManager`)
    (:`Is Not Valid`
      (`self.SetSpawnManager`))))

(event `RespawnPlayer`
  (params (Player :type "/Game/Blueprints/Player/MidVehicleBP/BP_MidVehicleWithTurret Object Reference"))
  (bind _asps_vehicle_state (cast `/Game/Game/PS_VehicleState` (`Pawn.PlayerState` Player)))
  (bind _spawnpoint (`/Game/Game/SpawnPoints/BP_TDMSpawnManager.GetAvailableSpawn` (`self.TDM_SpawnManager`) (`/Game/Game/PS_VehicleState.Team` _asps_vehicle_state)))
  (`SceneComponent.K2_SetWorldTransform` (`Actor.RootComponent` Player) (`SceneComponent.K2_GetComponentToWorld` (`/Game/Game/SpawnPoints/BP_SpawnPoint.SpawnPoint` _spawnpoint)) false false))

(fn `SetSpawnManager`
  (bind _outactors (`GameplayStatics.GetAllActorsOfClass` "/Game/Game/SpawnPoints/BP_TDMSpawnManager.BP_TDMSpawnManager_C"))
  (set `self.TDM_SpawnManager` (`|GetArrayItem` _outactors)))

(fn `UserConstructionScript`)