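; GM_FFAGameMode is the free-for-all game mode that builds the match leaderboard.
; CreateLeaderBoard makes a slot for each valid player with name, avatar, kills, deaths and assists.
; It bubble-sorts the slots by descending kills.
; On each sort pass, it also sends the slots to every player's PC_VehicleController through CreateFFALeaderBoard to create the client-side leaderboard.
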(fn `CreateLeaderBoard`
  (locals (PlayerSlots :type "Array of /Game/Game/LeaderboardSlot Structure") (unsorted :type Boolean))
  (bind _playerslots (`local.PlayerSlots`))
  ;[1 1 1] Create Player Slots for each player
  (bind _validplayerlist (`self.GetValidPlayerList`))
  (for _array_element _validplayerlist
    (`KismetArrayLibrary.Array_Add` (`local.PlayerSlots`) (make `/Game/Game/LeaderboardSlot` (`KismetTextLibrary.Conv_StringToText` (`PlayerState.GetPlayerName` _array_element)) (`/Game/Game/PS_VehicleState.PlayerAvatar` _array_element) (`/Game/Game/PS_VehicleState.Kills` _array_element) (`/Game/Game/PS_VehicleState.Deaths` _array_element) (`/Game/Game/PS_VehicleState.Assists` _array_element))))
  ;[1 1 1] Bubble Sort through num of kills
  (set `local.unsorted` true)
  (while (`local.unsorted`)
    (set `local.unsorted` false)
    (for _index (range (+ (- (`KismetArrayLibrary.Array_Length` (`local.PlayerSlots`)) 2) 1))
      (bind _returnvalue (+ _index 1))
      (if (< (`.Kills_5_6ECAB9414EB041C5101737AB1C1E4FA6` (break `/Game/Game/LeaderboardSlot` (`|GetArrayItem` _playerslots _index))) (`.Kills_5_6ECAB9414EB041C5101737AB1C1E4FA6` (break `/Game/Game/LeaderboardSlot` (`|GetArrayItem` _playerslots _returnvalue))))
        (set `local.unsorted` true)
        (`KismetArrayLibrary.Array_Swap` (`local.PlayerSlots`) _index _returnvalue)))
    ;[1 1 1] Create LeaderBoard in each clients machine
    (for _index_2 (range (`KismetArrayLibrary.Array_Length` (`GameStateBase.PlayerArray` (`GameplayStatics.GetGameState`))))
      (bind _aspc_vehicle_controller (cast `/Game/Game/PC_VehicleController` (`GameplayStatics.GetPlayerController` _index_2)))
      (`/Game/Game/PC_VehicleController.CreateFFALeaderBoard` _aspc_vehicle_controller (`local.PlayerSlots`)))))

(fn `UserConstructionScript`
  (`parent.UserConstructionScript`))