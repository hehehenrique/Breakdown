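; In-game game mode for a Carnage vs Breakdown vehicle combat match, running it from all-players-ready to game over.
; Once every player initialises, it builds scoreboards, then starts the game state, minimaps, vehicles and train carts.
; Kills update team totals on the game state.
; EndMatch snapshots stats into leaderboard slots that survive disconnects, bubble-sorts them by kills (Carnage gets only one pass), picks the winner and shows leaderboards after a delay.
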(event `OnAllPlayersReady`
  (`self.CreateScoreBoard`)
  (`self.BeginMatch`))

(event `self.UniqueInitialised`
  (params (VehicleState :type "/Game/Game/PS_VehicleState Object Reference"))
  (`parent.UniqueInitialised` VehicleState)
  (`/Game/Game/PS_VehicleState.LoadPlayerAvatar` VehicleState)
  (if (== (`KismetArrayLibrary.Array_Length` (`GameStateBase.PlayerArray` (`GameplayStatics.GetGameState`))) (`self.initialisedCount`))
    (`KismetSystemLibrary.PrintString` "ALL PLAYERS READY")
    (`self.OnAllPlayersReady`)))

(event `self.ReceiveBeginPlay`
  (`parent.ReceiveBeginPlay`)
  (bind _asbp_game_instance (cast `/Game/Game/BP_Game_Instance` (`GameplayStatics.GetGameInstance`)))
  (`MyOnlineGameInstance.UpdateServerVisibility` _asbp_game_instance false))

(event `BeginMatch`
  (set `self.matchRunning` true)
  (`/Game/Game/GameStates/GS_IngameGameState.BeginMatch` (`self.GetIngameGameState`) (`self.maxTime`))
  (`|ExecutionSequence`
    (:`then_0`
      (`self.InitialiseAllMinimaps`))
    (:`then_1`
      (bind _validplayerlist (`self.GetValidPlayerList`))
      (for _array_element _validplayerlist
        (`/Game/Blueprints/Player/MidVehicleBP/BP_BaseVehicle.OnMatchStarted` (`/Game/Game/PS_VehicleState.OwnedVehicle` _array_element))))
    (:`then_2`
      (bind _outactors (`GameplayStatics.GetAllActorsOfClass` "/Game/Blueprints/Train_Cart/BP_TrainCartManager.BP_TrainCartManager_C"))
      (`/Game/Blueprints/Train_Cart/BP_TrainCartManager.ActivateAllCarts` (`|GetArrayItem` _outactors)))))

(event `EndMatch`
  (params (EndGameReason :type "/Game/Game/EEndMatchReason Enum" :default "NewEnumerator0"))
  (set `self.matchRunning` false)
  (`/Game/Game/GameStates/GS_IngameGameState.ForceGameOver` (`self.GetIngameGameState`))
  (bind (_carnage _breakdown _winningteam) (`self.CreateLeaderBoard`))
  (`|ExecutionSequence`
    (:`then_0`
      ;[1 1 1] Disable Input on all vehicles
      (for _index (range (`self.m_playerCount`))
        (bind _aspc_vehicle_controller (cast `/Game/Game/PC_VehicleController` (`GameplayStatics.GetPlayerController` _index)))
        (`/Game/Game/PC_VehicleController.OnGameOver` _aspc_vehicle_controller)
        ;[1 1 1] Create Leader Board (gives time for it to load / initialize )
        (`/Game/Game/PC_VehicleController.CreateLeaderBoard` _aspc_vehicle_controller _carnage _breakdown _winningteam)))
    (:`then_2`
      (`KismetSystemLibrary.Delay` 3.0)
      (for _index_2 (range (`self.m_playerCount`))
        (bind _aspc_vehicle_controller_2 (cast `/Game/Game/PC_VehicleController` (`GameplayStatics.GetPlayerController` _index_2)))
        (`/Game/Game/PC_VehicleController.ShowLeaderBoard` _aspc_vehicle_controller_2)))))

(event `self.PlayerKilled`
  (params (VehicleState :type "/Game/Game/PS_VehicleState Object Reference"))
  ;[1 1 1] Player Killed
  (`parent.PlayerKilled` VehicleState)
  ;;[1 1 1] Update GameState Kill Counts
  (bind (_carnagekills _breakdownkills) (`self.Get Updated Kill Counters`))
  (bind _asgs_ingame_game_state (cast `/Game/Game/GameStates/GS_IngameGameState` (`GameplayStatics.GetGameState`)))
  (set `/Game/Game/GameStates/GS_IngameGameState.CarnageKillCount` _carnagekills _asgs_ingame_game_state)
  (set `/Game/Game/GameStates/GS_IngameGameState.BreakdownKillCount` _breakdownkills _asgs_ingame_game_state))

(fn `CreateLeaderBoard`
  (returns (Carnage :type "Array of /Game/Game/LeaderboardSlot Structure") (Breakdown :type "Array of /Game/Game/LeaderboardSlot Structure") (WinningTeam :type "/Game/Game/ETeam Enum"))
  (locals (CarnageStates :type "Array of /Game/Game/PS_VehicleState Object Reference") (BreakdownStates :type "Array of /Game/Game/PS_VehicleState Object Reference") (CarnageSlots :type "Array of /Game/Game/LeaderboardSlot Structure") (BreakdownSlots :type "Array of /Game/Game/LeaderboardSlot Structure") (unsorted :type Boolean :default true) (CarnageKills :type Integer) (BreakdownKills :type Integer))
  (bind _breakdownslots (`local.BreakdownSlots`))
  (bind _breakdownslots_2 (`local.BreakdownSlots`))
  (bind _carnageslots (`local.CarnageSlots`))
  (bind _carnageslots_2 (`local.CarnageSlots`))
  ;[1 1 1] Separate the 2 teams into arrays
  (bind _validplayerlist (`self.GetValidPlayerList`))
  (for _array_element _validplayerlist
    (switch `/Game/Game/ETeam` (`/Game/Game/PS_VehicleState.Team` _array_element)
      (:`NewEnumerator0`
        (`KismetArrayLibrary.Array_Add` (`local.CarnageStates`) _array_element))
      (:`NewEnumerator1`
        (`KismetArrayLibrary.Array_Add` (`local.BreakdownStates`) _array_element))))
  ;[1 1 1] Generate Leaderboard Slots to save important info for each player (this way it will stay saved even if the player leaves the session)
  (for _array_element_2 (`local.CarnageStates`)
    (`KismetArrayLibrary.Array_Add` (`local.CarnageSlots`) (make `/Game/Game/LeaderboardSlot` (`KismetTextLibrary.Conv_StringToText` (`PlayerState.GetPlayerName` _array_element_2)) (`/Game/Game/PS_VehicleState.PlayerAvatar` _array_element_2) (`/Game/Game/PS_VehicleState.Kills` _array_element_2) (`/Game/Game/PS_VehicleState.Deaths` _array_element_2) (`/Game/Game/PS_VehicleState.Assists` _array_element_2))))
  (for _array_element_3 (`local.BreakdownStates`)
    (`KismetArrayLibrary.Array_Add` (`local.BreakdownSlots`) (make `/Game/Game/LeaderboardSlot` (`KismetTextLibrary.Conv_StringToText` (`PlayerState.GetPlayerName` _array_element_3)) (`/Game/Game/PS_VehicleState.PlayerAvatar` _array_element_3) (`/Game/Game/PS_VehicleState.Kills` _array_element_3) (`/Game/Game/PS_VehicleState.Deaths` _array_element_3) (`/Game/Game/PS_VehicleState.Assists` _array_element_3))))
  ;[1 1 1] Bubble sort the Leaderboard Slots by highest kill count
  (set `local.unsorted` true)
  (while (`local.unsorted`)
    (set `local.unsorted` false)
    (for _index (range (+ (- (`KismetArrayLibrary.Array_Length` (`local.BreakdownSlots`)) 2) 1))
      (bind _returnvalue (+ _index 1))
      (if (< (`.Kills_5_6ECAB9414EB041C5101737AB1C1E4FA6` (break `/Game/Game/LeaderboardSlot` (`|GetArrayItem` _breakdownslots_2 _index))) (`.Kills_5_6ECAB9414EB041C5101737AB1C1E4FA6` (break `/Game/Game/LeaderboardSlot` (`|GetArrayItem` _breakdownslots_2 _returnvalue))))
        (set `local.unsorted` true)
        (`KismetArrayLibrary.Array_Swap` (`local.BreakdownSlots`) _index _returnvalue))))
  (set `local.unsorted` true)
  (while (`local.unsorted`)
    (for _index_2 (range (+ (- (`KismetArrayLibrary.Array_Length` (`local.CarnageSlots`)) 2) 1))
      (bind _returnvalue_2 (+ _index_2 1))
      (if (< (`.Kills_5_6ECAB9414EB041C5101737AB1C1E4FA6` (break `/Game/Game/LeaderboardSlot` (`|GetArrayItem` _carnageslots_2 _index_2))) (`.Kills_5_6ECAB9414EB041C5101737AB1C1E4FA6` (break `/Game/Game/LeaderboardSlot` (`|GetArrayItem` _carnageslots_2 _returnvalue_2))))
        (set `local.unsorted` true)
        (`KismetArrayLibrary.Array_Swap` (`local.CarnageSlots`) _index_2 _returnvalue_2)))
    ;[1 1 1] Compare total kills to determine winning team
    (for _array_element_4 (`local.CarnageSlots`)
      (set `local.CarnageKills` (+ (`local.CarnageKills`) (`.Kills_5_6ECAB9414EB041C5101737AB1C1E4FA6` (break `/Game/Game/LeaderboardSlot` _array_element_4)))))
    (for _array_element_5 (`local.BreakdownSlots`)
      (set `local.BreakdownKills` (+ (`local.BreakdownKills`) (`.Kills_5_6ECAB9414EB041C5101737AB1C1E4FA6` (break `/Game/Game/LeaderboardSlot` _array_element_5)))))
    (if (== (`local.CarnageKills`) (`local.BreakdownKills`))
      (return (`local.CarnageSlots`) (`local.BreakdownSlots`) "NewEnumerator2")
      (elif (> (`local.CarnageKills`) (`local.BreakdownKills`))
        (return _carnageslots _breakdownslots "NewEnumerator0")
        (else
          (return _carnageslots _breakdownslots "NewEnumerator1"))))))

(fn `CreateScoreBoard`
  (locals (RedStates :type "Array of /Game/Game/PS_VehicleState Object Reference") (BlueStates :type "Array of /Game/Game/PS_VehicleState Object Reference"))
  (bind _validplayerlist (`self.GetValidPlayerList`))
  (for _array_element _validplayerlist
    (switch `/Game/Game/ETeam` (`/Game/Game/PS_VehicleState.Team` _array_element)
      (:`NewEnumerator0`
        (`KismetArrayLibrary.Array_Add` (`local.RedStates`) _array_element))
      (:`NewEnumerator1`
        (`KismetArrayLibrary.Array_Add` (`local.BlueStates`) _array_element))))
  (for _index (range (`KismetArrayLibrary.Array_Length` _validplayerlist))
    (bind _aspc_vehicle_controller (cast `/Game/Game/PC_VehicleController` (`GameplayStatics.GetPlayerController` _index)))
    (`/Game/Game/PC_VehicleController.CreateScoreBoardWidget` _aspc_vehicle_controller (`local.RedStates`) (`local.BlueStates`))))

(fn `Get Updated Kill Counters`
  (returns (CarnageKills :type Integer) (BreakdownKills :type Integer))
  (locals (CarnageKillCount :type Integer) (BreakdownKillCount :type Integer))
  (bind _validplayerlist (`self.GetValidPlayerList`))
  (for _array_element _validplayerlist
    (switch `/Game/Game/ETeam` (`/Game/Game/PS_VehicleState.Team` _array_element)
      (:`NewEnumerator0`
        (bind _kills (`/Game/Game/PS_VehicleState.Kills` _array_element))
        (set `local.CarnageKillCount` (+ _kills (`local.CarnageKillCount`))))
      (:`NewEnumerator1`
        (set `local.BreakdownKillCount` (+ (`local.BreakdownKillCount`) _kills)))))
  (return (`local.CarnageKillCount`) (`local.BreakdownKillCount`)))

(fn `GetIngameGameState`
  (returns (IngameGS :type "/Game/Game/GameStates/GS_IngameGameState Object Reference"))
  (bind _asgs_ingame_game_state (cast `/Game/Game/GameStates/GS_IngameGameState` (`GameplayStatics.GetGameState`)))
  (return _asgs_ingame_game_state))

(fn `InitialiseAllMinimaps`
  (bind _validplayerlist (`self.GetValidPlayerList`))
  (for _array_element _validplayerlist
    (`/Game/Game/PC_VehicleController.InitialiseMinimap` (`/Game/Game/PS_VehicleState.OwningController` _array_element) _validplayerlist)))

(fn `UserConstructionScript`
  (`parent.UserConstructionScript`))