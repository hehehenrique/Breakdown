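; Online game mode for team-based vehicle combat that handles player setup, spawning, respawning and seamless level travel.
; Each player's vehicle spawns once replicated settings and team dispatchers on PS_VehicleState yield valid vehicle, turret and team, with possession on request.
; BP_TDMSpawnManager supplies team spawn points, and deaths start a respawn timer on the vehicle.
; It also serves team-assigned player lists to widgets and saves settings locally before travel.
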(event `RequestCurrentPlayerList`
  (params (VehicleCon :type "/Game/Game/PC_VehicleController Object Reference"))
  ;[1 1 1] Request Current Player List ( used for widgets )
  (bind _validplayerlist (`self.GetValidPlayerList`))
  (`/Game/Game/PC_VehicleController.ReceiveUpdatedPlayerList` VehicleCon _validplayerlist))

(event `self.ReceiveBeginPlay`
  ;[1 1 1] Initialise TDM Spawn Manager if needed
  (`/Engine/EditorBlueprintResources/StandardMacros.IsValid` (`self.TDM_SpawnManager`)
    (:`Is Not Valid`
      (`self.SetSpawnManager`))))

(event `InitiateSeamlessTravel`
  ;[1 1 1] Initiate Seamless Travel
  (for _index (range (`KismetArrayLibrary.Array_Length` (`GameStateBase.PlayerArray` (`GameplayStatics.GetGameState`))))
    (bind _aspc_vehicle_controller (cast `/Game/Game/PC_VehicleController` (`GameplayStatics.GetPlayerController` _index)))
    (`/Game/Game/PC_VehicleController.SaveInfoOnLocalMachine` _aspc_vehicle_controller) ; Force a local save of the owning vehicle's settings on each connected machine
    (`/Game/Game/PC_VehicleController.Teardown` _aspc_vehicle_controller))
  (`self.TravelToDesiredLevel`) ; Move to the new level, using seamless travel
)

(event `self.GenericPlayerInit`
  (params (Controller :type "Controller Object Reference"))
  ;[1 1 1] Generic Player Init (Runs on PostLogin and when new level is loaded)
  (bind _aspc_vehicle_controller (cast `/Game/Game/PC_VehicleController` Controller))
  (bind _asps_vehicle_state (cast `/Game/Game/PS_VehicleState` (`Controller.PlayerState` _aspc_vehicle_controller)))
  (add `/Game/Game/PS_VehicleState.VehicleSettingsDispatcher` _asps_vehicle_state (delegate `VehicleSettingsReceived`)) ; Bind an event that will fire when the VehicleSettings for this specific PlayerState are replicated
  (add `/Game/Game/PS_VehicleState.DefinedTeamDispatcher` _asps_vehicle_state (delegate `PlayerTeamDefined`))
  (set `/Game/Game/PS_VehicleState.OwningController` _aspc_vehicle_controller _asps_vehicle_state)
  (`/Game/Game/PC_VehicleController.UpdateRequest` _aspc_vehicle_controller) ; Request the vehicle controller to update its vehicle settings
)

(event `VehicleSettingsReceived`
  (params (VehicleState :type "/Game/Game/PS_VehicleState Object Reference"))
  ;[1 1 1] Generic Player Init (Runs on PostLogin and when new level is loaded)
  (`self.Try Initialise Player` VehicleState))

(event `PlayerTeamDefined`
  (params (VehicleState :type "/Game/Game/PS_VehicleState Object Reference"))
  ;[1 1 1] Generic Player Init (Runs on PostLogin and when new level is loaded)
  (`self.Try Initialise Player` VehicleState))

(event `InitialiseVehicle`
  (params (VehicleState :type "/Game/Game/PS_VehicleState Object Reference"))
  (bind _vehiclesettings (`/Game/Game/PS_VehicleState.VehicleSettings` VehicleState))
  ;[1 1 1] Initialise Vehicle
  ;;[1 1 1 1 14] Move to Available Spawn Point
  (bind _spawnt (`self.GetAvailableSpawnTransform` VehicleState))
  (bind _returnvalue (`|SpawnActorFromClass` (`.VehicleType_9_111BA6824FC48086422678BDF4F6F5CB` (break `/Game/Blueprints/CustomVehicleSetting` _vehiclesettings)) _spawnt "Undefined" "OverrideRootScale" VehicleState _vehiclesettings (`/Game/Game/PS_VehicleState.OwningController` VehicleState) null))
  (set `/Game/Game/PS_VehicleState.OwnedVehicle` _returnvalue VehicleState))

(event `UniqueInitialised`
  (params (VehicleState :type "/Game/Game/PS_VehicleState Object Reference"))
  ;[1 1 1] Unique Player Initialised
  (`/Engine/EditorBlueprintResources/StandardMacros.IncrementInt` (`self.initialisedCount`)
    (:`  `
      (`KismetSystemLibrary.PrintString` "initialised" true true (struct :`R` 1.0 :`G` 0.003583 :`B` 0.541 :`A` 1.0)))))

(event `PossessionRequested`
  (params (VehicleCon :type "/Game/Game/PC_VehicleController Object Reference") (BaseVehicle :type "/Game/Blueprints/Player/MidVehicleBP/BP_BaseVehicle Object Reference"))
  (`Controller.Possess` VehicleCon BaseVehicle))

(event `RespawnPlayer`
  (params (Player :type "/Game/Blueprints/Player/MidVehicleBP/BP_BaseVehicle Object Reference"))
  ;[1 1 1] Respawn Player
  (bind _asps_vehicle_state (cast `/Game/Game/PS_VehicleState` (`Pawn.PlayerState` Player)))
  (bind _spawnpoint (`/Game/Game/SpawnPoints/BP_TDMSpawnManager.GetAvailableSpawn` (`self.TDM_SpawnManager`) (`/Game/Game/PS_VehicleState.Team` _asps_vehicle_state)))
  (`PrimitiveComponent.SetPhysicsLinearVelocity` (`/Game/Blueprints/Player/MidVehicleBP/BP_BaseVehicle.SM_Body` Player) (0.0 0.0 0.0) false "None") ; Reset Velocity
  (`SceneComponent.K2_SetWorldTransform` (`Actor.RootComponent` Player) (`SceneComponent.K2_GetComponentToWorld` (`/Game/Game/SpawnPoints/BP_SpawnPoint.SpawnPoint` _spawnpoint)) false false) ; Move to spawn point
  (`/Game/Blueprints/Player/MidVehicleBP/BP_BaseVehicle.OnRespawn` Player))

(event `PlayerKilled`
  (params (VehicleState :type "/Game/Game/PS_VehicleState Object Reference"))
  ;[1 1 1] PlayerKilled
  (`|ExecutionSequence`
    (:`then_0`
      (`/Game/Blueprints/Player/MidVehicleBP/BP_BaseVehicle.BeginRespawnTimer` (`/Game/Game/PS_VehicleState.OwnedVehicle` VehicleState) (`self.RespawnTimer`)))
    (:`then_1`
      (`/Game/Game/PS_VehicleState.GotKilled` VehicleState))))

(fn `GetAvailableSpawnTransform`
  (params (VehicleState :type "/Game/Game/PS_VehicleState Object Reference"))
  (returns (SpawnT :type "Transform Structure"))
  (`/Engine/EditorBlueprintResources/StandardMacros.IsValid` (`self.TDM_SpawnManager`) ; Check if TDM Spawn Manager needs setting
    (:`Is Valid`
      _)
    (:`Is Not Valid`
      (`self.SetSpawnManager`)))
  (bind _spawnpoint (`/Game/Game/SpawnPoints/BP_TDMSpawnManager.GetAvailableSpawn` (`self.TDM_SpawnManager`) (`/Game/Game/PS_VehicleState.Team` VehicleState)))
  (return (`SceneComponent.K2_GetComponentToWorld` (`/Game/Game/SpawnPoints/BP_SpawnPoint.SpawnPoint` _spawnpoint))))

(fn `GetValidPlayerList`
  (returns (ValidPlayerList :type "Array of /Game/Game/PS_VehicleState Object Reference"))
  (locals (ValidPlayers :type "Array of /Game/Game/PS_VehicleState Object Reference"))
  (`|ExecutionSequence`
    (:`then_0`
      (for _array_element (`GameStateBase.PlayerArray` (`GameplayStatics.GetGameState`))
        (bind _asps_vehicle_state (cast `/Game/Game/PS_VehicleState` _array_element))
        (if (`|EnumInequality` (`/Game/Game/PS_VehicleState.Team` _asps_vehicle_state) "NewEnumerator2")
          (`KismetArrayLibrary.Array_Add` (`local.ValidPlayers`) _asps_vehicle_state))))
    (:`then_1`
      (return (`local.ValidPlayers`)))))

(fn `OnRep_initialisedCount`)

(fn `SetSpawnManager`
  (bind _outactors (`GameplayStatics.GetAllActorsOfClass` "/Game/Game/SpawnPoints/BP_TDMSpawnManager.BP_TDMSpawnManager_C"))
  (set `self.TDM_SpawnManager` (`|GetArrayItem` _outactors)))

(fn `Try Initialise Player`
  (params (VehicleState :type "/Game/Game/PS_VehicleState Object Reference"))
  (bind (_vehicletype _turret) (break `/Game/Blueprints/CustomVehicleSetting` (`/Game/Game/PS_VehicleState.VehicleSettings` VehicleState)))
  (if (and (`KismetSystemLibrary.IsValidClass` _vehicletype) (`KismetSystemLibrary.IsValidClass` _turret) (`|EnumInequality` (`/Game/Game/PS_VehicleState.Team` VehicleState) "NewEnumerator2") (not (`KismetSystemLibrary.IsValid` (`/Game/Game/PS_VehicleState.OwnedVehicle` VehicleState))))
    (`self.InitialiseVehicle` VehicleState)))

(fn `UserConstructionScript`)