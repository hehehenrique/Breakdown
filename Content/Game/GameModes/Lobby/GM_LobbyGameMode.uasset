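; Lobby game mode that keeps the server's visibility and player count up to date through BP_Game_Instance.
; On BeginPlay it casts the game instance, sets server visibility to true and passes it the current MPlayerCount.
; PostLogin and OnLogout share one update path that pushes MPlayerCount to the game instance again after calling their parent events.
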(event `self.ReceiveBeginPlay`
  (`parent.ReceiveBeginPlay`)
  (bind _asbp_game_instance (cast `/Game/Game/BP_Game_Instance` (`GameplayStatics.GetGameInstance`)))
  (`MyOnlineGameInstance.UpdateServerVisibility` _asbp_game_instance true)
  (`MyOnlineGameInstance.UpdateCurrentPlayers` _asbp_game_instance (`self.m_playerCount`)))

(event `self.K2_PostLogin`
  (params (NewPlayer :type "PlayerController Object Reference"))
  ;[1 1 1] Update Player Count
  (`parent.K2_PostLogin` NewPlayer)
  (bind _asbp_game_instance (cast `/Game/Game/BP_Game_Instance` (`GameplayStatics.GetGameInstance`) :!label _label))
  (`MyOnlineGameInstance.UpdateCurrentPlayers` _asbp_game_instance (`self.m_playerCount`)))

(event `self.K2_OnLogout`
  (params (ExitingController :type "Controller Object Reference"))
  ;[1 1 1] Update Player Count
  (`parent.K2_OnLogout` ExitingController)
  (goto _label))

(fn `UserConstructionScript`
  (`parent.UserConstructionScript`))