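; Game instance that persists player settings and vehicle/team state and handles online session events.
; Settings load from a save slot or get defaults, and saving writes graphics, sound and control structs back.
; Graphics settings apply through console commands for resolution and quality levels.
; Vehicle settings and team use a separate slot, while session teardown opens MainMenu behind a loading screen and failed connections show an error in the online menu.
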(event `self.OnDestroySessionComplete`
  (params (sessionName :type Name) (success :type Boolean))
  (`KismetSystemLibrary.PrintString` (`KismetStringLibrary.Conv_BoolToString` success) true true (struct :`R` 1.0 :`G` 0.11564 :`A` 1.0) 6.0)
  (if success
    (bind _aspc_vehicle_controller (cast `/Game/Game/PC_VehicleController` (`GameplayStatics.GetPlayerController` 0)))
    (`/Game/Game/PC_VehicleController.ShowLoadingScreen` _aspc_vehicle_controller)
    (`GameplayStatics.OpenLevel` "MainMenu")))

(event `self.ConnectionAttemptFailed`
  (params (reason :type "EConnectionError Enum" :default "SessionIsFull"))
  (bind _foundwidgets (`WidgetBlueprintLibrary.GetAllWidgetsOfClass` "/Game/MenuSystem/WBP_OnlineMainMenu.WBP_OnlineMainMenu_C"))
  (`/Game/UI/ConnectionState/WBP_ConnectionState.ShowError` (`/Game/MenuSystem/WBP_OnlineMainMenu.WBP_ConnectionFailed` (`|GetArrayItem` _foundwidgets)) reason))

(fn `ApplyGraphicsSettings`
  (params (GraphicSettings :type "/Game/UI/SettingsSaving/GraphicsSettingsStructure Structure"))
  (bind (_resolutionindex _aaindex _ppindex _shadowqualityindex _texturequalityindex _effectsqualityindex) (break `/Game/UI/SettingsSaving/GraphicsSettingsStructure` GraphicSettings))
  (bind _resolutions (`KismetSystemLibrary.GetSupportedFullscreenResolutions`))
  (bind (_x _y) (break `IntPoint` (`|GetArrayItem` _resolutions _resolutionindex)))
  (`KismetSystemLibrary.ExecuteConsoleCommand` (`KismetStringLibrary.Concat_StrStr` "r.setres " (`KismetStringLibrary.Conv_IntToString` _x) "x" (`KismetStringLibrary.Conv_IntToString` _y) "f") null)
  (`|ExecutionSequence`
    (:`then_0`
      (switch `/Game/UI/Enumerators/HighMediumLow_States` _aaindex
        (:`NewEnumerator0`
          (`KismetSystemLibrary.ExecuteConsoleCommand` "r.PostProcessAAQuality 6" null))
        (:`NewEnumerator1`
          (`KismetSystemLibrary.ExecuteConsoleCommand` "r.PostProcessAAQuality 4" null))
        (:`NewEnumerator2`
          (`KismetSystemLibrary.ExecuteConsoleCommand` "r.PostProcessAAQuality 2" null))))
    (:`then_1`
      (switch `/Game/UI/Enumerators/HighMediumLow_States` _ppindex
        (:`NewEnumerator0`
          (`KismetSystemLibrary.ExecuteConsoleCommand` "sg.PostProcessQuality 3" null))
        (:`NewEnumerator1`
          (`KismetSystemLibrary.ExecuteConsoleCommand` "sg.PostProcessQuality 2" null))
        (:`NewEnumerator2`
          (`KismetSystemLibrary.ExecuteConsoleCommand` "sg.PostProcessQuality 1" null))))
    (:`then_2`
      (switch `/Game/UI/Enumerators/HighMediumLow_States` _shadowqualityindex
        (:`NewEnumerator0`
          (`KismetSystemLibrary.ExecuteConsoleCommand` "sg.ShadowQuality 3" null))
        (:`NewEnumerator1`
          (`KismetSystemLibrary.ExecuteConsoleCommand` "sg.ShadowQuality 2" null))
        (:`NewEnumerator2`
          (`KismetSystemLibrary.ExecuteConsoleCommand` "sg.ShadowQuality 1" null))))
    (:`then_3`
      (switch `/Game/UI/Enumerators/HighMediumLow_States` _texturequalityindex
        (:`NewEnumerator0`
          (`KismetSystemLibrary.ExecuteConsoleCommand` "sg.TextureQuality 3" null))
        (:`NewEnumerator1`
          (`KismetSystemLibrary.ExecuteConsoleCommand` "sg.TextureQuality 2" null))
        (:`NewEnumerator2`
          (`KismetSystemLibrary.ExecuteConsoleCommand` "sg.TextureQuality 1" null))))
    (:`then_4`
      (switch `/Game/UI/Enumerators/HighMediumLow_States` _effectsqualityindex
        (:`NewEnumerator0`
          (`KismetSystemLibrary.ExecuteConsoleCommand` "sg.EffectsQuality 3" null))
        (:`NewEnumerator1`
          (`KismetSystemLibrary.ExecuteConsoleCommand` "sg.EffectsQuality 2" null))
        (:`NewEnumerator2`
          (`KismetSystemLibrary.ExecuteConsoleCommand` "sg.EffectsQuality 2" null))))))

(fn `DoesSavedSettingsExist`
  ;[1 1 1] Check to see if save settings exist
  (bind _returnvalue (`GameplayStatics.DoesSaveGameExist` (`self.SaveSettingsSlotName`)))
  (if _returnvalue
    ;[1 1 1] If true load and cast to settings save and reference to it
    (bind _returnvalue_2 (`GameplayStatics.LoadGameFromSlot` (`self.SaveSettingsSlotName`)))
    (bind _assettings_save (cast `/Game/UI/SettingsSaving/SettingsSave` _returnvalue_2))
    (set `self.SettingsSaveGame` _assettings_save)
    (else
      ;[1 1 1] If false, create save game, cast and reference to it and set default values for settings
      (bind _returnvalue_3 (`GameplayStatics.CreateSaveGameObject` "/Game/UI/SettingsSaving/SettingsSave.SettingsSave_C"))
      (bind _assettings_save_2 (cast `/Game/UI/SettingsSaving/SettingsSave` _returnvalue_3))
      (bind _output_get (set `self.SettingsSaveGame` _assettings_save_2))
      (`/Game/UI/SettingsSaving/SettingsSave.SetControlSettings` _output_get (make `/Game/UI/SettingsSaving/ControlSettingStructure` 1.0))
      (`/Game/UI/SettingsSaving/SettingsSave.SetSoundSettings` _output_get (make `/Game/UI/SettingsSaving/SoundSettingsStructure` 1.0 1.0 1.0))
      (bind _resolutions (`KismetSystemLibrary.GetSupportedFullscreenResolutions`))
      (`/Game/UI/SettingsSaving/SettingsSave.SetGraphicSettings` _output_get (make `/Game/UI/SettingsSaving/GraphicsSettingsStructure` (`KismetArrayLibrary.Array_LastIndex` _resolutions) "NewEnumerator1" "NewEnumerator1" "NewEnumerator1" "NewEnumerator1" "NewEnumerator1")))))

(fn `GetSavedPlayerStateInfo`
  (returns (Success :type Boolean) (VehicleSettings :type "/Game/Blueprints/CustomVehicleSetting Structure") (Team :type "/Game/Game/ETeam Enum"))
  (bind _returnvalue (`GameplayStatics.DoesSaveGameExist` (`self.VehicleStateSlotName`)))
  (if _returnvalue
    (bind _returnvalue_2 (`GameplayStatics.LoadGameFromSlot` (`self.VehicleStateSlotName`)))
    (bind _asvehicle_info_save (cast `/Game/Game/VehicleInfoSave` _returnvalue_2)
      (:`then`
        (return true (`/Game/Game/VehicleInfoSave.VehicleSettings` _asvehicle_info_save) (`/Game/Game/VehicleInfoSave.Team` _asvehicle_info_save)))
      (:`CastFailed`
        _)))
  (return false (struct) "NewEnumerator2"))

(fn `GetSavedSettings`
  (returns (SavedGraphicsSetting :type "/Game/UI/SettingsSaving/GraphicsSettingsStructure Structure") (SavedSoundSetting :type "/Game/UI/SettingsSaving/SoundSettingsStructure Structure") (SavedControlSetting :type "/Game/UI/SettingsSaving/ControlSettingStructure Structure"))
  (bind _settingssavegame (`self.SettingsSaveGame`))
  (return (`/Game/UI/SettingsSaving/SettingsSave.SavedGraphicsSetting` _settingssavegame) (`/Game/UI/SettingsSaving/SettingsSave.SavedSoundSetting` _settingssavegame) (`/Game/UI/SettingsSaving/SettingsSave.SavedControlSetting` _settingssavegame)))

(fn `SavePlayerStateInfo`
  (params (VehicleSettings :type "/Game/Blueprints/CustomVehicleSetting Structure") (ETeam :type "/Game/Game/ETeam Enum" :default "NewEnumerator2"))
  (bind _returnvalue (`GameplayStatics.CreateSaveGameObject` "/Game/Game/VehicleInfoSave.VehicleInfoSave_C"))
  (set `/Game/Game/VehicleInfoSave.Team` ETeam _returnvalue)
  (set `/Game/Game/VehicleInfoSave.VehicleSettings` VehicleSettings _returnvalue)
  (`GameplayStatics.SaveGameToSlot` _returnvalue (`self.VehicleStateSlotName`)))

(fn `SaveSettings`
  (params (GraphicSettings :type "/Game/UI/SettingsSaving/GraphicsSettingsStructure Structure") (SoundSettings :type "/Game/UI/SettingsSaving/SoundSettingsStructure Structure") (ControlSettings :type "/Game/UI/SettingsSaving/ControlSettingStructure Structure"))
  (bind _settingssavegame (`self.SettingsSaveGame`))
  (`/Game/UI/SettingsSaving/SettingsSave.SetGraphicSettings` _settingssavegame GraphicSettings)
  (`/Game/UI/SettingsSaving/SettingsSave.SetSoundSettings` _settingssavegame SoundSettings)
  (`/Game/UI/SettingsSaving/SettingsSave.SetControlSettings` _settingssavegame ControlSettings)
  (`GameplayStatics.SaveGameToSlot` _settingssavegame (`self.SaveSettingsSlotName`)))