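; Player controller that applies saved vehicle settings to the possessed BP_MidVehicleWithTurret.
; On BeginPlay it calls UpdateVehicleSettings, then passes the settings to the pawn's CustomSetupFromServer.
; UpdateVehicleSettings loads the VehicleSettingsSave slot if it exists, caches its settings on the controller and copies them to the controlled vehicle.
; Without a save, the controller's existing VehicleSettings value is used for setup.
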(event `self.ReceiveBeginPlay`
  (`self.UpdateVehicleSettings`)
  (bind _asbp_mid_vehicle_with_turret (cast `/Game/Blueprints/Player/MidVehicleBP/BP_MidVehicleWithTurret` (`self.K2_GetPawn`)))
  (`/Game/Blueprints/Player/MidVehicleBP/BP_MidVehicleWithTurret.CustomSetupFromServer` _asbp_mid_vehicle_with_turret (`self.VehicleSettings`)))

(event `UpdateVehicleSettings`
  (bind _returnvalue (`GameplayStatics.DoesSaveGameExist` "VehicleSettingsSave"))
  (if _returnvalue
    (bind _returnvalue_2 (`GameplayStatics.LoadGameFromSlot` "VehicleSettingsSave"))
    (bind _asvehicle_settings_save (cast `/Game/Game/VehicleSettingsSave` _returnvalue_2))
    (bind _output_get (set `self.VehicleSettings` (`/Game/Game/VehicleSettingsSave.VehicleSettings` _asvehicle_settings_save)))
    (bind _asbp_mid_vehicle_with_turret (cast `/Game/Blueprints/Player/MidVehicleBP/BP_MidVehicleWithTurret` (`self.K2_GetPawn`)))
    (set `/Game/Blueprints/Player/MidVehicleBP/BP_MidVehicleWithTurret.VehicleSettings` _output_get _asbp_mid_vehicle_with_turret)))

(fn `UserConstructionScript`)