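; Team deathmatch spawn manager that holds separate spawn point arrays for the Breakdown and Carnage teams.
; Each team's getter picks the first point that is neither occluded nor near enemies, optionally shuffling the array before returning.
; GetAvailableSpawn switches on team but only calls the Breakdown getter, and its return node is unconnected.
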(fn `GetAvailableBreakdownSpawn`
  (returns (BreakdownSpawn :type "/Game/Game/SpawnPoints/BP_SpawnPoint Object Reference"))
  ;[1 1 1] Loop through all elements, checking if there are any nearby enemies or if the spawn point area itself is occluded
  (for _array_element (`self.BreakdownSpawnPoints`)
    (bind _spawnoccluded (`/Game/Game/SpawnPoints/BP_SpawnPoint.IsSpawnOccluded` _array_element))
    (bind _enemiesnearby (`/Game/Game/SpawnPoints/BP_SpawnPoint.AreEnemiesNearby` _array_element))
    (if (`KismetMathLibrary.BooleanNOR` _enemiesnearby _spawnoccluded)
      (if (`self.shouldRandomize`)
        (`KismetArrayLibrary.Array_Shuffle` (`self.BreakdownSpawnPoints`)))
      (return _array_element))))

(fn `GetAvailableCarnageSpawn`
  (returns (CarnageSpawn :type "/Game/Game/SpawnPoints/BP_SpawnPoint Object Reference"))
  ;[1 1 1] Loop through all elements, checking if there are any nearby enemies or if the spawn point area itself is occluded
  (for _array_element (`self.CarnageSpawnPoints`)
    (bind _spawnoccluded (`/Game/Game/SpawnPoints/BP_SpawnPoint.IsSpawnOccluded` _array_element))
    (bind _enemiesnearby (`/Game/Game/SpawnPoints/BP_SpawnPoint.AreEnemiesNearby` _array_element))
    (if (`KismetMathLibrary.BooleanNOR` _enemiesnearby _spawnoccluded)
      (if (`self.shouldRandomize`)
        (`KismetArrayLibrary.Array_Shuffle` (`self.CarnageSpawnPoints`)))
      (return _array_element))))

(fn `GetAvailableSpawn`
  (params (Team :type "/Game/Game/ETeam Enum" :default "NewEnumerator2"))
  (returns (SpawnPoint :type "/Game/Game/SpawnPoints/BP_SpawnPoint Object Reference"))
  (switch `/Game/Game/ETeam` Team
    (:`NewEnumerator1`
      (`self.GetAvailableBreakdownSpawn`))))

(fn `UserConstructionScript`
  (`parent.UserConstructionScript`))