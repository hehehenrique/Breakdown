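; Free-for-all spawn manager that picks an unoccluded spawn point.
; The construction script collects every BP_SpawnPoint actor in the level into SpawnPoints.
; GetAvailableSpawn returns the first unoccluded point from a shuffled SpawnPoints when randomizing, otherwise from FirstSpawnPoints in stored order.
; The Team input is unused, and there is no fallback when every candidate is occluded.
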(fn `GetAvailableSpawn`
  (params (Team :type "/Game/Game/ETeam Enum" :default "NewEnumerator2"))
  (returns (SpawnPoint :type "/Game/Game/SpawnPoints/BP_SpawnPoint Object Reference"))
  ;[1 1 1] Loop through all elements, checking if there are any nearby enemies nearby
  (if (`self.shouldRandomize`)
    (`KismetArrayLibrary.Array_Shuffle` (`self.SpawnPoints`)) ; Randomize order
    (for _array_element (`self.SpawnPoints`)
      (bind _spawnoccluded (`/Game/Game/SpawnPoints/BP_SpawnPoint.IsSpawnOccluded` _array_element))
      (if (not _spawnoccluded)
        (return _array_element)))
    (else
      (for _array_element_2 (`self.FirstSpawnPoints`)
        (bind _spawnoccluded_2 (`/Game/Game/SpawnPoints/BP_SpawnPoint.IsSpawnOccluded` _array_element_2))
        (if (not _spawnoccluded_2)
          (return _array_element_2))))))

(fn `UserConstructionScript`
  (`parent.UserConstructionScript`)
  (bind _outactors (`GameplayStatics.GetAllActorsOfClass` "/Game/Game/SpawnPoints/BP_SpawnPoint.BP_SpawnPoint_C"))
  (for _array_element _outactors
    (`KismetArrayLibrary.Array_Add` (`self.SpawnPoints`) _array_element)))