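; BP_SpawnPoint is a team-assigned vehicle spawn point that reports whether it is blocked or has enemies nearby.
; AreEnemiesNearby scans BP_BaseVehicle actors overlapping EnemyCheck and returns true if any has a PS_VehicleState team different from the point's Team.
; IsSpawnOccluded returns true when any BP_BaseVehicle overlaps SpawnOcclusion, regardless of team.
; Both checks query overlaps when called, and the construction script is empty.
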(fn `AreEnemiesNearby`
  (returns (enemiesNearby :type Boolean))
  (locals (foundEnemy :type Boolean))
  (`|ExecutionSequence`
    (:`then_0`
      (for _array_element (`PrimitiveComponent.GetOverlappingActors` (`self.EnemyCheck`) "/Game/Blueprints/Player/MidVehicleBP/BP_BaseVehicle.BP_BaseVehicle_C")
        (bind _asbp_base_vehicle (cast `/Game/Blueprints/Player/MidVehicleBP/BP_BaseVehicle` _array_element))
        (bind _asps_vehicle_state (cast `/Game/Game/PS_VehicleState` (`Pawn.PlayerState` _asbp_base_vehicle)))
        (if (!= (`/Game/Game/PS_VehicleState.Team` _asps_vehicle_state) (`self.Team`))
          (set `local.foundEnemy` true)
          (break))))
    (:`then_1`
      (return (`local.foundEnemy`)))))

(fn `IsSpawnOccluded`
  (returns (SpawnOccluded :type Boolean))
  (return (> (`KismetArrayLibrary.Array_Length` (`PrimitiveComponent.GetOverlappingActors` (`self.SpawnOcclusion`) "/Game/Blueprints/Player/MidVehicleBP/BP_BaseVehicle.BP_BaseVehicle_C")) 0)))

(fn `UserConstructionScript`)