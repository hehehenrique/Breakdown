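; Spawn manager that picks an available spawn point for a player, based on the game state (FFA or TDM, lobby or in-game) and team.
; TDM returns the first Carnage or Breakdown point with no occlusion or nearby enemies, optionally shuffling that team's list for later calls.
; FFA merges both lists, optionally shuffles them, and returns the first unoccluded point without checking for enemies.
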(fn `GetAvailableBreakdownSpawn`
  (returns (BreakdownSpawn :type "/Game/Game/SpawnPoints/BP_SpawnPoint Object Reference"))
  ;[1 1 1] Loop through all elements, checking if there are any nearby enemies or if the spawn point area itself is occluded
  (for _array_element (`self.BreakdownSpawnPoints`)
    (bind _spawnoccluded (`/Game/Game/SpawnPoints/BP_SpawnPoint.IsSpawnOccluded` _array_element))
    (bind _enemiesnearby (`/Game/Game/SpawnPoints/BP_SpawnPoint.AreEnemiesNearby` _array_element))
    (if (`KismetMathLibrary.BooleanNOR` _enemiesnearby _spawnoccluded)
      (if (`self.shouldRandomize`)
        (`KismetArrayLibrary.Array_Shuffle` (`self.BreakdownSpawnPoints`)))
      (return _array_element))))

(fn `GetAvailableCarnageSpawn`
  (returns (CarnageSpawn :type "/Game/Game/SpawnPoints/BP_SpawnPoint Object Reference"))
  ;[1 1 1] Loop through all elements, checking if there are any nearby enemies or if the spawn point area itself is occluded
  (for _array_element (`self.CarnageSpawnPoints`)
    (bind _spawnoccluded (`/Game/Game/SpawnPoints/BP_SpawnPoint.IsSpawnOccluded` _array_element))
    (bind _enemiesnearby (`/Game/Game/SpawnPoints/BP_SpawnPoint.AreEnemiesNearby` _array_element))
    (if (`KismetMathLibrary.BooleanNOR` _enemiesnearby _spawnoccluded)
      (if (`self.shouldRandomize`)
        (`KismetArrayLibrary.Array_Shuffle` (`self.CarnageSpawnPoints`)))
      (return _array_element))))

(fn `GetAvailableFFASpawn`
  (returns (Spawn :type "/Game/Game/SpawnPoints/BP_SpawnPoint Object Reference"))
  (locals (AllSpawnPoints :type "Array of /Game/Game/SpawnPoints/BP_SpawnPoint Object Reference"))
  ;[1 1 1] Loop through all elements, checking if there are any nearby enemies nearby
  ;;[1 1 1] Create AllSpawnPoints Array
  (bind _output_get (set `local.AllSpawnPoints` (`self.BreakdownSpawnPoints`)))
  (for _array_element (`self.CarnageSpawnPoints`)
    (`KismetArrayLibrary.Array_Add` _output_get _array_element))
  (`|ExecutionSequence`
    (:`then_0`
      (if (`self.shouldRandomize`)
        (`KismetArrayLibrary.Array_Shuffle` (`local.AllSpawnPoints`)) ; Randomize order
      ))
    (:`then_1`
      (for _array_element_2 (`local.AllSpawnPoints`)
        (bind _spawnoccluded (`/Game/Game/SpawnPoints/BP_SpawnPoint.IsSpawnOccluded` _array_element_2))
        (if (not _spawnoccluded)
          (return _array_element_2))))))

(fn `GetAvailableSpawn`
  (params (Team :type "/Game/Game/ETeam Enum" :default "NewEnumerator0"))
  (returns (SpawnPoint :type "/Game/Game/SpawnPoints/BP_SpawnPoint Object Reference"))
  (switch `/Game/Game/GameStates/EGameStateClass` (`/Game/Blueprints/OnlineFunctionLib.GetGameStateClass`)
    (:`NewEnumerator0`
      _)
    (:`NewEnumerator1`
      _)
    (:`NewEnumerator2`
      (switch `/Game/Game/ETeam` Team :!label _label
        (:`NewEnumerator0`
          (bind _carnagespawn (`self.GetAvailableCarnageSpawn`))
          (return _carnagespawn))
        (:`NewEnumerator1`
          (bind _breakdownspawn (`self.GetAvailableBreakdownSpawn`))
          (return _breakdownspawn))))
    (:`NewEnumerator3`
      (goto _label)))
  (bind _spawn (`self.GetAvailableFFASpawn`))
  (return _spawn))

(fn `UserConstructionScript`)