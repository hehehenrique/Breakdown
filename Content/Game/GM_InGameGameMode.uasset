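; In-game GameMode for a team vehicle combat match that starts play once every player is initialised and tracks match state.
; When all players are ready it builds red and blue scoreboard widgets on each vehicle controller, activates the train cart manager's carts and starts the GameState timer.
; On each kill it re-sums player kills per team into the GameState's Carnage and Breakdown counters.
; Ending the match forces game over on the GameState.
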(event `OnAllPlayersReady`
  (`self.CreateScoreBoard`)
  (`self.BeginMatch`)
  (`/Game/Game/GS_InGameGameState.StartTimer` (`self.GetIngameGameState`) (`self.maxTime`)))

(event `self.UniqueInitialised`
  (params (VehicleState :type "/Game/Game/PS_VehicleState Object Reference"))
  (`parent.UniqueInitialised` VehicleState)
  (if (== (`KismetArrayLibrary.Array_Length` (`GameStateBase.PlayerArray` (`GameplayStatics.GetGameState`))) (`self.initialisedCount`))
    (`KismetSystemLibrary.PrintString` "ALL PLAYERS READY")
    (`self.OnAllPlayersReady`)))

(event `BeginMatch`
  (set `self.matchRunning` true)
  (bind _outactors (`GameplayStatics.GetAllActorsOfClass` "/Game/Blueprints/Train_Cart/BP_TrainCartManager.BP_TrainCartManager_C"))
  (`/Game/Blueprints/Train_Cart/BP_TrainCartManager.ActivateAllCarts` (`|GetArrayItem` _outactors)))

(event `EndMatch`
  (params (EndGameReason :type "/Game/Game/EEndMatchReason Enum" :default "NewEnumerator0"))
  (set `self.matchRunning` false)
  (`/Game/Game/GS_InGameGameState.ForceGameOver` (`self.GetIngameGameState`))
  (for _index (range (`KismetArrayLibrary.Array_Length` (`GameStateBase.PlayerArray` (`GameplayStatics.GetGameState`))))
    (cast `/Game/Game/PC_VehicleController` (`GameplayStatics.GetPlayerController` _index)))
  (`KismetSystemLibrary.PrintString` "GAME OVER"))

(event `self.PlayerKilled`
  (params (VehicleState :type "/Game/Game/PS_VehicleState Object Reference"))
  ;[1 1 1] Player Killed
  (`parent.PlayerKilled` VehicleState)
  ;;[1 1 1] Update GameState Kill Counts
  (bind (_carnagekills _breakdownkills) (`self.Get Updated Kill Counters`))
  (bind _asgs_ingame_game_state (cast `/Game/Game/GS_InGameGameState` (`GameplayStatics.GetGameState`)))
  (set `/Game/Game/GS_InGameGameState.CarnageKillCount` _carnagekills _asgs_ingame_game_state)
  (set `/Game/Game/GS_InGameGameState.BreakdownKillCount` _breakdownkills _asgs_ingame_game_state))

(fn `CreateScoreBoard`
  (locals (RedStates :type "Array of /Game/Game/PS_VehicleState Object Reference") (BlueStates :type "Array of /Game/Game/PS_VehicleState Object Reference"))
  (bind _validplayerlist (`self.GetValidPlayerList`))
  (for _array_element _validplayerlist
    (switch `/Game/Game/ETeam` (`/Game/Game/PS_VehicleState.Team` _array_element)
      (:`NewEnumerator0`
        (`KismetArrayLibrary.Array_Add` (`local.RedStates`) _array_element))
      (:`NewEnumerator1`
        (`KismetArrayLibrary.Array_Add` (`local.BlueStates`) _array_element))))
  (for _index (range (`KismetArrayLibrary.Array_Length` _validplayerlist))
    (bind _aspc_vehicle_controller (cast `/Game/Game/PC_VehicleController` (`GameplayStatics.GetPlayerController` _index)))
    (`/Game/Game/PC_VehicleController.CreateScoreBoardWidget` _aspc_vehicle_controller (`local.RedStates`) (`local.BlueStates`))))

(fn `Get Updated Kill Counters`
  (returns (CarnageKills :type Integer) (BreakdownKills :type Integer))
  (locals (CarnageKillCount :type Integer) (BreakdownKillCount :type Integer))
  (bind _validplayerlist (`self.GetValidPlayerList`))
  (for _array_element _validplayerlist
    (switch `/Game/Game/ETeam` (`/Game/Game/PS_VehicleState.Team` _array_element)
      (:`NewEnumerator0`
        (bind _kills (`/Game/Game/PS_VehicleState.Kills` _array_element))
        (set `local.CarnageKillCount` (+ _kills (`local.CarnageKillCount`))))
      (:`NewEnumerator1`
        (set `local.BreakdownKillCount` (+ (`local.BreakdownKillCount`) _kills)))))
  (return (`local.CarnageKillCount`) (`local.BreakdownKillCount`)))

(fn `GetIngameGameState`
  (returns (IngameGS :type "/Game/Game/GS_InGameGameState Object Reference"))
  (bind _asgs_ingame_game_state (cast `/Game/Game/GS_InGameGameState` (`GameplayStatics.GetGameState`)))
  (return _asgs_ingame_game_state))

(fn `UserConstructionScript`
  (`parent.UserConstructionScript`))