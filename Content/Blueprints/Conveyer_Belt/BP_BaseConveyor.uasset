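; Base conveyor belt actor that moves whatever overlaps its TransportOverlap along the TransportDirection forward vector.
; Every Tick it loops over overlapping actors, skipping other conveyors.
; Vehicles get an acceleration force on SMBody, scaled by BeltSpeed, delta time and PlayerMoveForce, with their name printed for debugging.
; All other actors are offset directly by BeltSpeed and delta time, without sweep.
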(event `self.ReceiveTick`
  (params (DeltaSeconds :type "Float (single-precision)"))
  (bind _returnvalue (* (`SceneComponent.GetForwardVector` (`self.TransportDirection`)) (* DeltaSeconds (`self.Belt_Speed`))))
  ;[1 1 1] For each loop runs on every tick and checks all overlapping actors and moves them
  (for _array_element (`PrimitiveComponent.GetOverlappingActors` (`self.TransportOverlap`) null)
    (cast `/Game/Blueprints/Conveyer_Belt/BP_BaseConveyor` _array_element ; Check that isn't another conveyor belt
      (:`CastFailed`
        (bind _asbp_base_vehicle (cast `/Game/Blueprints/Player/MidVehicleBP/BP_BaseVehicle` _array_element)
          (:`then`
            ;;[1 1 1] If is vehicle
            (`PrimitiveComponent.AddForce` (`/Game/Blueprints/Player/MidVehicleBP/BP_BaseVehicle.SM_Body` _asbp_base_vehicle) (* _returnvalue (* (`self.PlayerMoveForce`) 100.0)) "None" true)
            (`KismetSystemLibrary.PrintString` (`KismetSystemLibrary.GetDisplayName` _asbp_base_vehicle) true true (struct :`G` 0.66 :`B` 1.0 :`A` 1.0) (`GameplayStatics.GetWorldDeltaSeconds`)))
          (:`CastFailed`
            ;;[1 1 1] If isn't vehicle
            (`self.K2_AddActorWorldOffset` _array_element _returnvalue false false)))))))

(fn `UserConstructionScript`)