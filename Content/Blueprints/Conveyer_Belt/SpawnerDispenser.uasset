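; Conveyor belt spawner dispenser that spawns an actor at its own location with a random rotation.
; It spawns once on BeginPlay through SpawnerSetup.
; Tick polls the IsAlive flag on a referenced destroyer dispenser; when false, it starts a looping five-second timer on SpawnerSetup, sets the flag back to true and prints a respawn message.
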(event `self.ReceiveBeginPlay`
  (`self.SpawnerSetup`))

(event `self.ReceiveTick`
  (params (DeltaSeconds :type "Float (single-precision)"))
  (if (not (`/Game/Blueprints/Conveyer_Belt/DestroyerDispenser.isAlive` (`self.DestroyerDispenserRef`)))
    (`KismetSystemLibrary.K2_SetTimer` null "SpawnerSetup" 5.0 true)
    (set `/Game/Blueprints/Conveyer_Belt/DestroyerDispenser.isAlive` true (`self.DestroyerDispenserRef`))
    (`KismetSystemLibrary.PrintString` "Respawn")))

(event `SpawnerSetup`
  (`self.SpawnItems`))

(fn `SpawnItems`
  (`|SpawnActorFromClass` "/Game/Blueprints/Conveyer_Belt/Item.Item_C" (`KismetMathLibrary.MakeTransform` (`self.K2_GetActorLocation`) (`KismetMathLibrary.RandomRotator` true)) "Undefined" "OverrideRootScale" null null))

(fn `UserConstructionScript`)