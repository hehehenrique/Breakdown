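; BP_Roller_Medium_Open is a medium open roller conveyor that carries overlapping actors along its transport direction.
; Each tick it loops over actors in TransportOpenOverlap, skipping other conveyors, and moves them along TransportOpenDirection's forward vector, scaled by BeltSpeed and delta time.
; Vehicles get a physics force on their body mesh, further scaled by PlayerMoveForce, while other actors are offset directly without sweeping.
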(event `self.ReceiveTick`
  (params (DeltaSeconds :type "Float (single-precision)"))
  (bind _returnvalue (* (`SceneComponent.GetForwardVector` (`self.TransportOpenDirection`)) (* DeltaSeconds (`self.Belt_Speed`))))
  (`parent.ReceiveTick` DeltaSeconds)
  ;[1 1 1] For each loop runs on every tick and checks all overlapping actors and moves them
  (for _array_element (`PrimitiveComponent.GetOverlappingActors` (`self.TransportOpenOverlap`) null)
    (cast `/Game/Blueprints/Conveyer_Belt/BP_BaseConveyor` _array_element ; Check that isn't another conveyor belt
      (:`CastFailed`
        (bind _asbp_base_vehicle (cast `/Game/Blueprints/Player/MidVehicleBP/BP_BaseVehicle` _array_element)
          (:`then`
            ;;[1 1 1] If is vehicle
            (`PrimitiveComponent.AddForce` (`/Game/Blueprints/Player/MidVehicleBP/BP_BaseVehicle.SM_Body` _asbp_base_vehicle) (* _returnvalue (* (`self.PlayerMoveForce`) 100000.0)) "None" false))
          (:`CastFailed`
            ;;[1 1 1] If isn't vehicle
            (`self.K2_AddActorWorldOffset` _array_element _returnvalue false false)))))))

(fn `UserConstructionScript`
  (`parent.UserConstructionScript`))