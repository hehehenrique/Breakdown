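; Track spline Blueprint that builds a rail track along an editable spline in its construction script.
; When Debug is off, it applies the CloseLoop setting and divides the spline length by a mesh Length to get the segment count.
; Each segment adds a shadowless, collidable spline mesh using RailMesh, bent between positions sampled by distance, with tangents scaled by a Tangent multiplier.
; BeginPlay is empty.
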(event `self.ReceiveBeginPlay`)

(fn `UserConstructionScript`
  (bind _track_spline (`self.Track_Spline`))
  (bind _length (`self.Length`))
  (if (not (`self.Debug`))
    (`SplineComponent.SetClosedLoop` (`self.Track_Spline`) (`self.Close Loop?`) true)
    ;[1 1 1] For loop for multiple spline points
    (for _index (range (+ (`.ReturnValue` (`KismetMathLibrary.FMod` (`SplineComponent.GetSplineLength` (`self.Track_Spline`)) (`self.Length`))) 1))
      ;[1 1 1] Adds the spline mesh components
      (bind _returnvalue (`AddComponent|NODE_AddSplineMeshComponent-2`))
      ;[1 1 1] Sets any static mesh to the target
      (`PrimitiveComponent.SetCastShadow` _returnvalue false)
      (`StaticMeshComponent.SetStaticMesh` _returnvalue (`self.Rail Mesh`))
      (bind _returnvalue_2 (* _index _length))
      (bind _returnvalue_3 (+ _returnvalue_2 _length))
      ;[1 1 1] Go's through the start and end position of points and tangents
      (`SplineMeshComponent.SetStartAndEnd` _returnvalue (`SplineComponent.GetLocationAtDistanceAlongSpline` _track_spline _returnvalue_2 "Local") (* (`SplineComponent.GetTangentAtDistanceAlongSpline` _track_spline _returnvalue_2 "Local") (`self.Tangent`)) (`SplineComponent.GetLocationAtDistanceAlongSpline` _track_spline _returnvalue_3 "Local") (* (`SplineComponent.GetTangentAtDistanceAlongSpline` _track_spline _returnvalue_3 "Local") (`self.Tangent`)) true)
      ;[1 1 1] Enables collision through mesh
      (`PrimitiveComponent.SetCollisionEnabled` _returnvalue "QueryAndPhysics"))))