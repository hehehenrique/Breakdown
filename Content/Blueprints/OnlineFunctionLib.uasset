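; Blueprint function library with two team checks that report whether two vehicles, or two vehicle states, count as opponents.
; Both return true whenever the game state casts to GS_FFAState, so free-for-all treats every pair as opposing.
; Otherwise they return true only when the Team values differ, with VehicleCompareTeam reading Team through each vehicle's GetVehicleState.
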(fn `StateCompareTeam`
  (params (VehicleState1 :type "/Game/Game/PS_VehicleState Object Reference (by ref)") (VehicleState2 :type "/Game/Game/PS_VehicleState Object Reference (by ref)"))
  (returns (Enemies :type Boolean))
  (cast `/Game/Game/GameStates/GS_FFAState` (`GameplayStatics.GetGameState` (`local.__WorldContext`))
    (:`then`
      (return true))
    (:`CastFailed`
      (return (`|EnumInequality` (`/Game/Game/PS_VehicleState.Team` VehicleState1) (`/Game/Game/PS_VehicleState.Team` VehicleState2))))))

(fn `VehicleCompareTeam`
  (params (BaseVehicle1 :type "/Game/Blueprints/Player/MidVehicleBP/BP_BaseVehicle Object Reference (by ref)") (BaseVehicle2 :type "/Game/Blueprints/Player/MidVehicleBP/BP_BaseVehicle Object Reference (by ref)"))
  (returns (Enemies :type Boolean))
  (cast `/Game/Game/GameStates/GS_FFAState` (`GameplayStatics.GetGameState` (`local.__WorldContext`))
    (:`then`
      (return true))
    (:`CastFailed`
      (return (`|EnumInequality` (`/Game/Game/PS_VehicleState.Team` (`/Game/Blueprints/Player/MidVehicleBP/BP_BaseVehicle.GetVehicleState` BaseVehicle1 BaseVehicle1)) (`/Game/Game/PS_VehicleState.Team` (`/Game/Blueprints/Player/MidVehicleBP/BP_BaseVehicle.GetVehicleState` BaseVehicle2 BaseVehicle2)))))))