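; Behavior Tree task that steers a BP_BaseAI pawn toward a location read from a Blackboard vector key.
; Each tick it stores the final target, finds a navmesh path synchronously and sets the pawn's immediate target to the path's second point, leaving movement to the pawn.
; It draws debug shapes for both targets and finishes successfully once the pawn reports arrival.
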(event `self.ReceiveTickAI`
  (params (OwnerController :type "AIController Object Reference") (ControlledPawn :type "Pawn Object Reference") (DeltaSeconds :type "Float (single-precision)"))
  (bind _ai_pawn (`self.AI_Pawn`))
  (bind _returnvalue (`BTFunctionLibrary.GetBlackboardValueAsVector` (`self.Vector`)))
  (bind _asbp_base_ai (cast `/Game/Blueprints/AI/BP_BaseAI` ControlledPawn))
  (bind _output_get (set `self.AI_Pawn` _asbp_base_ai))
  (set `/Game/Blueprints/AI/BP_BaseAI.FinalTarget` _returnvalue _output_get)
  (`KismetSystemLibrary.DrawDebugSphere` _returnvalue 100.0 12 (struct :`R` 1.0 :`A` 1.0) 0.0001 10.0)
  (bind _returnvalue_2 (`NavigationSystemV1.FindPathToLocationSynchronously` (`Actor.K2_GetActorLocation` (`self.AI_Pawn`)) _returnvalue null null))
  (bind _output_get_2 (set `/Game/Blueprints/AI/BP_BaseAI.TargetPosition` (`|GetArrayItem` (`NavigationPath.PathPoints` _returnvalue_2) 1) _ai_pawn))
  (`KismetSystemLibrary.DrawDebugLine` (`Actor.K2_GetActorLocation` (`self.AI_Pawn`)) _output_get_2 (struct :`R` 0.07265 :`G` 1.0 :`A` 1.0) 0.0001 15.0)
  (bind _arrivedatlocation (`/Game/Blueprints/AI/BP_BaseAI.Check if Arrived at Target` _ai_pawn))
  (if _arrivedatlocation
    (`KismetSystemLibrary.PrintString` "Arrived at target" true true (struct :`G` 1.0 :`B` 0.065497 :`A` 1.0) 5.0)
    (`self.FinishExecute` true)))