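; Behavior tree task that completes when a BP_BaseAI pawn arrives at a Blackboard vector location.
; Each tick it casts the controlled pawn, measures its distance to that location and prints the value on screen for debugging.
; Within a fixed radius it clears the pawn's StartMoving flag and finishes successfully; it starts no movement itself and has no failure path.
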(event `self.ReceiveTickAI`
  (params (OwnerController :type "AIController Object Reference") (ControlledPawn :type "Pawn Object Reference") (DeltaSeconds :type "Float (single-precision)"))
  (bind _asbp_base_ai (cast `/Game/Blueprints/AI/BP_BaseAI` ControlledPawn))
  (bind _output_get (set `self.AI_Pawn` _asbp_base_ai))
  (bind _returnvalue (`KismetMathLibrary.VSize` (- (`Actor.K2_GetActorLocation` _output_get) (`BTFunctionLibrary.GetBlackboardValueAsVector` (`self.Vector`)))))
  (`KismetSystemLibrary.PrintString` (`KismetStringLibrary.Conv_DoubleToString` _returnvalue) true true (struct :`G` 0.66 :`B` 1.0 :`A` 1.0) 1e-05)
  (if (< _returnvalue 150.0)
    (set `/Game/Blueprints/AI/BP_BaseAI.startMoving` false (`self.AI_Pawn`))
    (`self.FinishExecute` true)))