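; BP_BaseAI is a base AI hover vehicle that drives a physics body toward a target position.
; On BeginPlay it overrides the body's mass and scales four corner hover components' spring and damping to that mass.
; Each tick it updates speed and, while StartMoving is set, turns forward and right dot products to the target into throttle force and yaw torque.
; An arrival check, uncalled here, clears StartMoving near the target.
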(event `self.ReceiveBeginPlay`
  ;[1 1 1] Setting up Hover Components Array
  (set `self.HoverComponentsArray` (`|MakeArray` (`self.BP_MidAIHoverComponentFL`) (`self.BP_MidAIHoverComponentFR`) (`self.BP_MidAIHoverComponentRR`) (`self.BP_MidAIHoverComponentRL`)))
  ;[1 1 1] Setting mass of the vehicle from mass variable
  (`PrimitiveComponent.SetMassOverrideInKg` (`self.SM_Body`) "None" (`self.Mass`) true)
  (`self.SetHoverComponents`))

(event `self.ReceiveTick`
  (params (DeltaSeconds :type "Float (single-precision)"))
  (`|ExecutionSequence`
    (:`then_0`
      (`self.Calculate Speed KMH`))
    (:`then_1`
      (if (`self.startMoving`)
        (`self.NavigateToTarget` (`self.TargetPosition`))))))

(fn `AddAcceleration`
  (params (`Input Throttle` :type "Float (double-precision)"))
  (locals (AccelerationScalingValue :type "Float (double-precision)" :default 10000.0) (AccelerationIncrement :type "Float (double-precision)"))
  (set `local.AccelerationIncrement` (* `Input Throttle` (`local.AccelerationScalingValue`)))
  (`PrimitiveComponent.AddForce` (`self.SM_Body`) (* (`self.GetActorForwardVector`) (* (`local.AccelerationIncrement`) (`self.Acceleration`))) "None" false))

(fn `AddTorque`
  (params (`Steering Input` :type "Float (double-precision)"))
  (locals (TorqueScalingValue :type "Float (double-precision)" :default 100000000.0) (TorqueIncrement :type "Float (double-precision)"))
  (set `local.TorqueIncrement` (* `Steering Input` (`local.TorqueScalingValue`)))
  (`PrimitiveComponent.AddTorqueInDegrees` (`self.SM_Body`) (* (`self.GetActorUpVector`) (* (`local.TorqueIncrement`) (`self.Steering`))) "None" false))

(fn `Calculate Speed KMH`
  (set `self.speedKMH` (/ (`KismetMathLibrary.VSize` (`self.GetVelocity`)) 27.778)))

(fn `CalculateThrottleAndSteering`
  (params (TargetPosition :type "Vector Structure"))
  (locals (TargetPos :type "Vector Structure"))
  (set `local.TargetPos` TargetPosition)
  (bind _direction (`self.CheckIfForward/Back` self (`local.TargetPos`)))
  (set `self.ThrottleInput` _direction)
  (bind _direction_2 (`self.CheckIfLeft/Right` self (`local.TargetPos`)))
  (set `self.SteeringInput` _direction_2))

(fn `Check if Arrived at Target`
  (returns (ArrivedAtLocation :type Boolean))
  (bind _returnvalue (< (`KismetMathLibrary.VSize` (- (`self.K2_GetActorLocation`) (`self.TargetPosition`))) 100.0))
  (if _returnvalue
    (set `self.startMoving` false))
  (return _returnvalue))

(fn `CheckIfForward/Back`
  (params (Actor :type "Actor Object Reference") (TargetPosition :type "Vector Structure"))
  (returns (Direction :type "Float (double-precision)"))
  (return (`KismetMathLibrary.Dot_VectorVector` (`KismetMathLibrary.Normal` (- TargetPosition (`self.K2_GetActorLocation` Actor))) (`self.GetActorForwardVector` Actor))))

(fn `CheckIfLeft/Right`
  (params (Actor :type "Actor Object Reference") (TargetPosition :type "Vector Structure"))
  (returns (Direction :type "Float (double-precision)"))
  (return (`KismetMathLibrary.Dot_VectorVector` (`KismetMathLibrary.Normal` (- TargetPosition (`self.K2_GetActorLocation` Actor))) (`self.GetActorRightVector` Actor))))

(fn `NavigateToTarget`
  (params (TargetPosition :type "Vector Structure"))
  (`self.CalculateThrottleAndSteering` TargetPosition)
  (`self.AddAcceleration` (`self.ThrottleInput`))
  (`self.AddTorque` (`self.SteeringInput`)))

(fn `SetHoverComponents`
  (locals (MinimalSpringCoefficientPer1KG :type "Float (double-precision)" :default 25.0) (MinimalDampingCoefficientPer1KG :type "Float (double-precision)" :default 1.0))
  ;[1 1 1] Setting enough force to the hover components to keep the vehicle up based on its mass
  (for _array_element (`self.HoverComponentsArray`)
    (set `/Game/Blueprints/AI/MidAIHoverComponent_BP.SpringCoefficient` (* (`self.Mass`) (`local.MinimalSpringCoefficientPer1KG`)) _array_element)
    (set `/Game/Blueprints/AI/MidAIHoverComponent_BP.DampingCoefficient` (* (`self.Mass`) (`local.MinimalDampingCoefficientPer1KG`)) _array_element)))

(fn `UserConstructionScript`)