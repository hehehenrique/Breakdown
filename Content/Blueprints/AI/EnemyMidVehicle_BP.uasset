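; EnemyMidVehicle_BP is a mid-size AI enemy hover vehicle held up by four corner hover components.
; On BeginPlay it gathers the front and rear hover components into an array and overrides the body mesh's mass from the Mass variable.
; SetHoverComponents then scales each component's spring and damping coefficients by that mass, using per-kilogram minimums, so the suspension force matches the vehicle's weight.
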(event `self.ReceiveBeginPlay`
  ;[1 1 1] Setting up Hover Components Array
  (set `self.HoverComponentsArray` (`|MakeArray` (`self.BP_MidAIHoverComponentFL`) (`self.BP_MidAIHoverComponentFR`) (`self.BP_MidAIHoverComponentRR`) (`self.BP_MidAIHoverComponentRL`)))
  ;[1 1 1] Setting mass of the vehicle from mass variable
  (`PrimitiveComponent.SetMassOverrideInKg` (`self.SM_Body`) "None" (`self.Mass`) true)
  (`self.SetHoverComponents`))

(fn `SetHoverComponents`
  (locals (MinimalSpringCoefficientPer1KG :type "Float (double-precision)" :default 25.0) (MinimalDampingCoefficientPer1KG :type "Float (double-precision)" :default 1.0))
  ;[1 1 1] Setting enough force to the hover components to keep the vehicle up based on its mass
  (for _array_element (`self.HoverComponentsArray`)
    (set `/Game/Blueprints/AI/MidAIHoverComponent_BP.SpringCoefficient` (* (`self.Mass`) (`local.MinimalSpringCoefficientPer1KG`)) _array_element)
    (set `/Game/Blueprints/AI/MidAIHoverComponent_BP.DampingCoefficient` (* (`self.Mass`) (`local.MinimalDampingCoefficientPer1KG`)) _array_element)))

(fn `UserConstructionScript`)