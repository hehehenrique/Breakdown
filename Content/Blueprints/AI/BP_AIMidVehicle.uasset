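; BP_AIMidVehicle is a physics-driven AI hover vehicle that can steer itself toward a target position.
; On BeginPlay it overrides body mass and scales the spring and damping of four corner hover components by that mass.
; GoToTargetPosition takes dot products of the target direction with the forward and right vectors, feeding AddThrottle and AddTorque.
; These apply scaled force along the forward axis and torque around the up axis.
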(event `self.ReceiveBeginPlay`
  ;[1 1 1] Setting up Hover Components Array
  (set `self.HoverComponentsArray` (`|MakeArray` (`self.BP_MidAIHoverComponentFL`) (`self.BP_MidAIHoverComponentFR`) (`self.BP_MidAIHoverComponentRR`) (`self.BP_MidAIHoverComponentRL`)))
  ;[1 1 1] Setting mass of the vehicle from mass variable
  (`PrimitiveComponent.SetMassOverrideInKg` (`self.SM_Body`) "None" (`self.Mass`) true)
  (`self.SetHoverComponents`))

(fn `AddThrottle`
  (params (`Input Throttle` :type "Float (double-precision)"))
  (locals (ThrottleScalingValue :type "Float (double-precision)" :default 10000.0) (Throttle :type "Float (double-precision)"))
  (set `local.Throttle` (* `Input Throttle` (`local.ThrottleScalingValue`)))
  (`PrimitiveComponent.AddForce` (`self.SM_Body`) (* (`self.GetActorForwardVector`) (`local.Throttle`)) "None" false))

(fn `AddTorque`
  (params (`Input Torque` :type "Float (double-precision)"))
  (locals (TorqueScalingValue :type "Float (double-precision)" :default 100000000.0) (Torque :type "Float (double-precision)"))
  (set `local.Torque` (* `Input Torque` (`local.TorqueScalingValue`)))
  (`PrimitiveComponent.AddTorqueInDegrees` (`self.SM_Body`) (* (`self.GetActorUpVector`) (`local.Torque`)) "None" false))

(fn `CheckIfForward/Back`
  (params (Actor :type "Actor Object Reference") (TargetPosition :type "Vector Structure"))
  (returns (Direction :type "Float (double-precision)"))
  (return (`KismetMathLibrary.Dot_VectorVector` (`KismetMathLibrary.Normal` (- TargetPosition (`self.K2_GetActorLocation` Actor))) (`self.GetActorForwardVector` Actor))))

(fn `CheckIfLeft/Right`
  (params (Actor :type "Actor Object Reference") (TargetPosition :type "Vector Structure"))
  (returns (Direction :type "Float (double-precision)"))
  (return (`KismetMathLibrary.Dot_VectorVector` (`KismetMathLibrary.Normal` (- TargetPosition (`self.K2_GetActorLocation` Actor))) (`self.GetActorRightVector` Actor))))

(fn `Go to Target Position`
  (params (TargetPosition :type "Vector Structure"))
  (locals (TargetPos :type "Vector Structure"))
  (set `local.TargetPos` TargetPosition)
  (bind _direction (`self.CheckIfForward/Back` self (`local.TargetPos`)))
  (bind _direction_2 (`self.CheckIfLeft/Right` self (`local.TargetPos`)))
  (`self.AddThrottle` (* _direction 700.0))
  (`self.AddTorque` (* _direction_2 400.0)))

(fn `SetHoverComponents`
  (locals (MinimalSpringCoefficientPer1KG :type "Float (double-precision)" :default 25.0) (MinimalDampingCoefficientPer1KG :type "Float (double-precision)" :default 1.0))
  ;[1 1 1] Setting enough force to the hover components to keep the vehicle up based on its mass
  (for _array_element (`self.HoverComponentsArray`)
    (set `/Game/Blueprints/AI/MidAIHoverComponent_BP.SpringCoefficient` (* (`self.Mass`) (`local.MinimalSpringCoefficientPer1KG`)) _array_element)
    (set `/Game/Blueprints/AI/MidAIHoverComponent_BP.DampingCoefficient` (* (`self.Mass`) (`local.MinimalDampingCoefficientPer1KG`)) _array_element)))

(fn `UserConstructionScript`)