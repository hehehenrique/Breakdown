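; Train cart that rides a track spline, carrying a pickup and flinging it with a catapult.
; A timeline drives spline position and rotation, with play rate scaled to a set duration.
; Station overlaps run a speed-change timeline that scales play rate and audio volume, attaching the sphere-detected pickup via an event track.
; Catapult-point overlaps release the pickup with physics and swing the catapult mesh out and back.
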(event `Activate`
  (bind _cart_movement (`self.Cart Movement`))
  (bind _returnvalue (`TimelineComponent.GetTimelineLength` _cart_movement))
  ;[1 1 1] Event BeginPlay -> Set the play rate of the cart, then check if there is a cart active on level
  (`TimelineComponent.SetPlayRate` _cart_movement (/ _returnvalue (`self.Duration`)))
  (if (`self.IsCartActive`)
    (`TimelineComponent.SetNewTime` (`self.Cart Movement`) (* (`self.PositionCart`) _returnvalue))
    (`self.Move Train Cart`)))

(event `Move Train Cart`
  (bind _returnvalue (`KismetMathLibrary.Lerp` 0.0 (`SplineComponent.GetSplineLength` (`/Game/Blueprints/Rail_Track_Spline/Track_Spline.Track_Spline` (`self.Spline Reference`))) (`self.SplineProgress`)))
  ;[1 1 1] Move Train Cart Event -> Timeline to move cart - Timeline to slow down and speed up when stopped
  (bind (_direction _progress) (`Timeline|Cart Movement`)
    (:`Update`
      (set `self.SplineProgress` _progress)
      (`self.K2_SetActorLocationAndRotation` (`SplineComponent.GetLocationAtDistanceAlongSpline` (`/Game/Blueprints/Rail_Track_Spline/Track_Spline.Track_Spline` (`self.Spline Reference`)) _returnvalue "World") (`SplineComponent.GetRotationAtDistanceAlongSpline` (`/Game/Blueprints/Rail_Track_Spline/Track_Spline.Track_Spline` (`self.Spline Reference`)) _returnvalue "World")))))

(event `self.Mesh Collision Box.OnComponentBeginOverlap`
  (params (OverlappedComponent :type "PrimitiveComponent Object Reference") (OtherActor :type "Actor Object Reference") (OtherComp :type "PrimitiveComponent Object Reference") (OtherBodyIndex :type Integer) (bFromSweep :type Boolean) (SweepResult :type "HitResult Structure (by ref)"))
  ;[1 1 1] Move Train Cart Event -> Timeline to move cart - Timeline to slow down and speed up when stopped
  (if (not (`self.isSlowingDown`))
    (cast `/Game/Blueprints/Train_Cart/Station` OtherActor)
    (set `self.isSlowingDown` true)
    (bind (_direction _speed) (`Timeline|SpeedChange` :!via `PlayFromStart`)
      (:`Update`
        (bind _output_get (set `self.PlayRateMult` _speed))
        (`AudioComponent.SetVolumeMultiplier` (`self.Minecart Audio`) _output_get)
        (`TimelineComponent.SetPlayRate` (`self.Cart Movement`) (* (/ (`TimelineComponent.GetTimelineLength` (`self.Cart Movement`)) (`self.Duration`)) (`self.PlayRateMult`))))
      (:`Finished`
        (set `self.isSlowingDown` false))
      (:`AttachEvent`
        (`self.AttachPickUp`)))))

(event `Catapult Start`
  ;[1 1 1] Custom Event to start Catapult Animation
  (`self.DetachPickUp`)
  (bind (_direction _progression_anim) (`Timeline|Catapult Animation` :!via `PlayFromStart`)
    (:`Update`
      (`SceneComponent.K2_SetRelativeRotation` (`self.Catapult Mesh`) (`KismetMathLibrary.RLerp` (struct :`Yaw` -180.0 :`Roll` 90.0) (struct :`Yaw` -180.0 :`Roll` 160.0) _progression_anim) false false))
    (:`Finished`
      (switch `ETimelineDirection` _direction
        (:`Forward`
          (`TimelineComponent.ReverseFromEnd` (`self.Catapult Animation`)))))))

(event `self.Train_Cart.OnComponentBeginOverlap`
  (params (OverlappedComponent :type "PrimitiveComponent Object Reference") (OtherActor :type "Actor Object Reference") (OtherComp :type "PrimitiveComponent Object Reference") (OtherBodyIndex :type Integer) (bFromSweep :type Boolean) (SweepResult :type "HitResult Structure (by ref)"))
  ;[1 1 1] If the cart is overlapping the catapult point then play the custom event
  (cast `/Game/Blueprints/Train_Cart/BP_Pickup_Catapult_Point` OtherActor)
  (`self.Catapult Start`))

(event `self.Sphere.OnComponentBeginOverlap`
  (params (OverlappedComponent :type "PrimitiveComponent Object Reference") (OtherActor :type "Actor Object Reference") (OtherComp :type "PrimitiveComponent Object Reference") (OtherBodyIndex :type Integer) (bFromSweep :type Boolean) (SweepResult :type "HitResult Structure (by ref)"))
  (`/Engine/EditorBlueprintResources/StandardMacros.IsValid` (`self.AttachedPickUp`)
    (:`Is Not Valid`
      (bind _asbp_base_pick_up (cast `/Game/Blueprints/PickUps/BP_Base_PickUp` OtherActor))
      (set `self.AttachedPickUp` _asbp_base_pick_up))))

(fn `AttachPickUp`
  (`/Engine/EditorBlueprintResources/StandardMacros.IsValid` (`self.AttachedPickUp`)
    (:`Is Valid`
      (`self.K2_AttachToActor` (`self.AttachedPickUp`) self "None" "KeepWorld" "KeepWorld" "KeepWorld" true)
      (`PrimitiveComponent.SetSimulatePhysics` (`/Game/Blueprints/PickUps/BP_Base_PickUp.Sphere` (`self.AttachedPickUp`)) false))))

(fn `DetachPickUp`
  (`/Engine/EditorBlueprintResources/StandardMacros.IsValid` (`self.AttachedPickUp`)
    (:`Is Valid`
      (`self.K2_DetachFromActor` (`self.AttachedPickUp`) "KeepWorld" "KeepWorld" "KeepWorld")
      (`PrimitiveComponent.SetSimulatePhysics` (`/Game/Blueprints/PickUps/BP_Base_PickUp.Sphere` (`self.AttachedPickUp`)) true)
      (set `self.AttachedPickUp` null))))

(fn `UserConstructionScript`)