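; Base projectile fired by vehicles, damaging other vehicles and pushing or damaging world objects it strikes.
; Vehicle overlaps run a backward sphere sweep for an accurate impact point, then call GotShot with curve-based distance falloff damage.
; Bounces apply impulses to physics bodies and radius damage to destructible meshes.
; Hits, spawning inside the owner vehicle, or lifetime expiry hide and disable the projectile before delayed destruction.
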(event `StartBulletLifetime`
  ;[1 1 1] StartBulletLifetime
  (`KismetSystemLibrary.Delay` (`self.GetDespawnTime`))
  (`self.DelayedDestroyProjectile`))

(event `self.ReceiveBeginPlay`
  ;[1 1 1] BEGIN PLAY
  (`self.CheckInitialOverlap`)
  (`self.StartBulletLifetime`))

(event `DelayedDestroyProjectile`
  ;[1 1 1] DelayedDestroyProjectile
  (`self.SetActorEnableCollision` false)
  (`SceneComponent.SetVisibility` (`self.ProjectileMesh`) false false)
  (`ActorComponent.SetActive` (`self.ProjectileMovement`) false true)
  (`KismetSystemLibrary.Delay` 2.0)
  (`self.K2_DestroyActor`))

(event `self.ProjectileCollision.OnComponentBeginOverlap`
  (params (OverlappedComponent :type "PrimitiveComponent Object Reference") (OtherActor :type "Actor Object Reference") (OtherComp :type "PrimitiveComponent Object Reference") (OtherBodyIndex :type Integer) (bFromSweep :type Boolean) (SweepResult :type "HitResult Structure (by ref)"))
  ;[1 1 1] On Begin Overlap ( Vehicles )
  (`self.OnBeginOverlap` OtherActor))

(event `self.ProjectileMovement.OnProjectileBounce`
  (params (ImpactResult :type "HitResult Structure (by ref)") (ImpactVelocity :type "Vector Structure (by ref)"))
  ;[1 1 1] On Projectile Bounce ( World )
  (`self.OnBounce` ImpactResult_ImpactPoint ImpactResult_HitComponent))

(fn `CheckInitialOverlap`
  (locals (shouldDestroySelf :type Boolean))
  (for _array_element (`PrimitiveComponent.GetOverlappingActors` (`self.ProjectileCollision`) "/Game/Blueprints/Player/MidVehicleBP/BP_BaseVehicle.BP_BaseVehicle_C")
    (if (== _array_element (`self.ownerVehicle`))
      (set `local.shouldDestroySelf` true)))
  (if (`local.shouldDestroySelf`)
    (`self.DelayedDestroyProjectile`)))

(fn `GetDamageFromDistance`
  (params (WorldImpactLoc :type "Vector Structure"))
  (returns (Damage :type "Float (double-precision)"))
  (return (`CurveFloat.GetFloatValue` (`self.DamageCurve`) (`KismetMathLibrary.VSize` (- WorldImpactLoc (`self.InitialWorldLoc`))))))

(fn `GetDespawnTime`
  (returns (bulletLifetime :type "Float (double-precision)"))
  (bind (_mintime _maxtime) (`CurveBase.GetTimeRange` (`self.DamageCurve`)))
  (if (and (<= (`CurveFloat.GetFloatValue` (`self.DamageCurve`) _maxtime) 10.0) (`self.shouldDespawnQuick`))
    (return (/ _maxtime (`self.TravelSpeed`)))
    (else
      (return 3.0))))

(fn `OnBeginOverlap`
  (params (OtherActor :type "Actor Object Reference"))
  (locals (VehicleHit :type "/Game/Blueprints/Player/MidVehicleBP/BP_BaseVehicle Object Reference"))
  (bind _ownervehicle (`self.ownerVehicle`))
  (bind _returnvalue (`SceneComponent.K2_GetComponentLocation` (`self.ProjectileCollision`)))
  (bind _returnvalue_2 (`SceneComponent.GetForwardVector` (`self.ProjectileCollision`)))
  (`|ExecutionSequence`
    (:`then_0`
      ;[1 1 1] Set VehicleHit
      (if (`self.IsChildActor` OtherActor)
        (bind _asbp_base_vehicle (cast `/Game/Blueprints/Player/MidVehicleBP/BP_BaseVehicle` (`self.GetParentActor` OtherActor)))
        (set `local.VehicleHit` _asbp_base_vehicle)
        (else
          (bind _asbp_base_vehicle_2 (cast `/Game/Blueprints/Player/MidVehicleBP/BP_BaseVehicle` OtherActor))
          (set `local.VehicleHit` _asbp_base_vehicle_2))))
    (:`then_1`
      ;[1 1 1] Check if isnt overlapping own vehicle
      (if (!= (`local.VehicleHit`) (`self.ownerVehicle`))
        ;[1 1 1] CCD sweep ( to get accurate point of impact )
        (bind (_outhit _returnvalue_3) (`KismetSystemLibrary.SphereTraceSingleForObjects` (- _returnvalue (* _returnvalue_2 (* (`self.TravelSpeed`) (`GameplayStatics.GetWorldDeltaSeconds`)))) (+ _returnvalue _returnvalue_2) (`SphereComponent.SphereRadius` (`self.ProjectileCollision`)) (`|MakeArray` "ObjectTypeQuery5" :!type "EObjectTypeQuery Enum") true (`|MakeArray` _ownervehicle (`/Game/Blueprints/Player/MidVehicleBP/BP_BaseVehicle.GetCustomTurret` _ownervehicle) :!type "Actor Object Reference") "None" true (struct :`R` 1.0 :`A` 1.0) (struct :`G` 1.0 :`A` 1.0) 60.0))
        (if _returnvalue_3
          (bind _asbp_base_vehicle_3 (cast `/Game/Blueprints/Player/MidVehicleBP/BP_BaseVehicle` (`self.GetOwner` (`self.GetOwner`)))) ; Get vehicle which shot this projectile ( the agressor )
          (`/Game/Blueprints/Player/MidVehicleBP/BP_BaseVehicle.GotShot` (`local.VehicleHit`) (`self.GetDamageFromDistance` (`.Location` (`GameplayStatics.BreakHitResult` _outhit))) _outhit (`self.GetActorForwardVector`) (`self.VehicleImpactStrength`) _asbp_base_vehicle_3) ; Call GotShot on VehicleHit
        )))
    (:`then_2`
      (`self.DelayedDestroyProjectile`))))

(fn `OnBounce`
  (params (ImpactResultImpactPoint :type "Vector Structure") (ImpactResultHitComponent :type "PrimitiveComponent Object Reference"))
  (`|ExecutionSequence`
    (:`then_0`
      (`/Engine/EditorBlueprintResources/StandardMacros.IsValid` ImpactResultHitComponent
        (:`Is Valid`
          (`|ExecutionSequence`
            (:`then_0`
              ;[1 1 1] Apply Force on Actors Simulating Physics
              (if (`SceneComponent.IsSimulatingPhysics` ImpactResultHitComponent "None")
                (`PrimitiveComponent.AddImpulseAtLocation` ImpactResultHitComponent (* (`self.GetActorForwardVector`) (`self.WorldImpactStrength`)) ImpactResultImpactPoint "None")))
            (:`then_1`
              ;[1 1 1] Apply Damage to Destructible Meshes
              (bind _asdestructible_component (cast `DestructibleComponent` ImpactResultHitComponent))
              (`DestructibleComponent.ApplyRadiusDamage` _asdestructible_component (`self.DMDamage`) ImpactResultImpactPoint 30.0 10.0 true))))))
    (:`then_1`
      (`self.DelayedDestroyProjectile`))))

(fn `UserConstructionScript`
  (set `MovementComponent.Velocity` (`KismetMathLibrary.MakeVector` (`self.TravelSpeed`)) (`self.ProjectileMovement`)) ; SET VELOCITY
  (set `self.InitialWorldLoc` (`SceneComponent.K2_GetComponentLocation` (`self.RootComponent`))))