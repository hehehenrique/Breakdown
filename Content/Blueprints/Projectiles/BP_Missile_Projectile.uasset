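; Missile projectile that explodes on bouncing or on hitting a vehicle other than its owner's, then destroys itself after a delay.
; An overlap sphere tracks nearby vehicles, and the explosion fires separate world and vehicle radial impulses with VFX and sound.
; Tracked vehicles take curve-based damage by distance, credited to the firing vehicle.
; On overlap, a backward-offset sphere sweep acts as CCD to move the missile to the accurate impact point.
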(event `self.ReceiveBeginPlay`
  (`parent.ReceiveBeginPlay`)
  (for _array_element (`PrimitiveComponent.GetOverlappingActors` (`self.VehicleOverlap`) "/Game/Blueprints/Player/MidVehicleBP/BP_BaseVehicle.BP_BaseVehicle_C")
    (bind _asbp_base_vehicle (cast `/Game/Blueprints/Player/MidVehicleBP/BP_BaseVehicle` _array_element))
    (`self.AddToOverlapped` _asbp_base_vehicle)))

(event `self.VehicleOverlap.OnComponentBeginOverlap`
  (params (OverlappedComponent :type "PrimitiveComponent Object Reference") (OtherActor :type "Actor Object Reference") (OtherComp :type "PrimitiveComponent Object Reference") (OtherBodyIndex :type Integer) (bFromSweep :type Boolean) (SweepResult :type "HitResult Structure (by ref)"))
  (bind _asbp_base_vehicle (cast `/Game/Blueprints/Player/MidVehicleBP/BP_BaseVehicle` OtherActor))
  (`self.AddToOverlapped` _asbp_base_vehicle))

(event `self.VehicleOverlap.OnComponentEndOverlap`
  (params (OverlappedComponent :type "PrimitiveComponent Object Reference") (OtherActor :type "Actor Object Reference") (OtherComp :type "PrimitiveComponent Object Reference") (OtherBodyIndex :type Integer))
  (bind _asbp_base_vehicle (cast `/Game/Blueprints/Player/MidVehicleBP/BP_BaseVehicle` OtherActor))
  (`self.RemoveFromOverlapped` _asbp_base_vehicle))

(fn `AddToOverlapped`
  (params (Vehicle :type "/Game/Blueprints/Player/MidVehicleBP/BP_BaseVehicle Object Reference"))
  (if (not (`KismetArrayLibrary.Array_Contains` (`self.OverlappedVehicles`) Vehicle))
    (`KismetArrayLibrary.Array_Add` (`self.OverlappedVehicles`) Vehicle)))

(fn `Explode`
  (`|ExecutionSequence`
    (:`then_0`
      ;[1 1 1] Apply Forces
      (`RadialForceComponent.FireImpulse` (`self.VehicleRadialForce`))
      (`RadialForceComponent.FireImpulse` (`self.WorldRadialForce`)))
    (:`then_1`
      (for _array_element (`self.OverlappedVehicles`)
        (bind _returnvalue (* (`CurveFloat.GetFloatValue` (`self.DamageCurve`) (* (/ (`KismetMathLibrary.VSize` (- (`SceneComponent.K2_GetComponentLocation` (`Actor.RootComponent` _array_element)) (`SceneComponent.K2_GetComponentLocation` (`self.RootComponent`)))) (`SphereComponent.SphereRadius` (`self.VehicleOverlap`))) 100.0)) 0.01 (`self.ExplosionMaxDamage`)))
        (if (< 0.0 _returnvalue)
          (bind _asbp_base_vehicle (cast `/Game/Blueprints/Player/MidVehicleBP/BP_BaseVehicle` (`self.GetOwner` (`self.GetOwner`))))
          (`/Game/Blueprints/Player/MidVehicleBP/BP_BaseVehicle.GotImpacted` :`self` _array_element :`Damage` _returnvalue :`Agressor` _asbp_base_vehicle))))
    (:`then_2`
      ;[1 1 1] Play VFX and Sound
      (`ActorComponent.Activate` (`self.VFXExplosion`) true)
      (`GameplayStatics.PlaySound2D` "/Game/Sounds/Cannon_Sounds/Launcher/Launcher_Shot_2.Launcher_Shot_2" 1.0 1.0 0.0 null null))))

(fn `OnBeginOverlap`
  (params (OtherActor :type "Actor Object Reference"))
  (locals (VehicleHit :type "/Game/Blueprints/Player/MidVehicleBP/BP_BaseVehicle Object Reference"))
  (bind _ownervehicle (`self.ownerVehicle`))
  (bind _returnvalue (`SceneComponent.K2_GetComponentLocation` (`self.ProjectileCollision`)))
  (bind _returnvalue_2 (`SceneComponent.GetForwardVector` (`self.ProjectileCollision`)))
  (`|ExecutionSequence`
    (:`then_0`
      ;[1 1 1] Set VehicleHit
      (if (`self.IsChildActor` OtherActor)
        (bind _asbp_base_vehicle (cast `/Game/Blueprints/Player/MidVehicleBP/BP_BaseVehicle` (`self.GetParentActor` OtherActor)))
        (set `local.VehicleHit` _asbp_base_vehicle)
        (else
          (bind _asbp_base_vehicle_2 (cast `/Game/Blueprints/Player/MidVehicleBP/BP_BaseVehicle` OtherActor))
          (set `local.VehicleHit` _asbp_base_vehicle_2))))
    (:`then_1`
      ;[1 1 1] Check if isnt overlapping own vehicle
      (if (!= (`local.VehicleHit`) (`self.ownerVehicle`))
        ;[1 1 1] CCD sweep ( to get accurate point of impact )
        (bind (_outhit _returnvalue_3) (`KismetSystemLibrary.SphereTraceSingleForObjects` (- _returnvalue (* _returnvalue_2 (* (`self.TravelSpeed`) (`GameplayStatics.GetWorldDeltaSeconds`)))) (+ _returnvalue _returnvalue_2) (`SphereComponent.SphereRadius` (`self.ProjectileCollision`)) (`|MakeArray` "ObjectTypeQuery5" :!type "EObjectTypeQuery Enum") true (`|MakeArray` _ownervehicle (`/Game/Blueprints/Player/MidVehicleBP/BP_BaseVehicle.GetCustomTurret` _ownervehicle) :!type "Actor Object Reference") "None" true (struct :`R` 1.0 :`A` 1.0) (struct :`G` 1.0 :`A` 1.0) 60.0))
        (if _returnvalue_3
          (`|ExecutionSequence`
            (:`then_0`
              (`self.K2_SetActorLocation` (`.Location` (`GameplayStatics.BreakHitResult` _outhit))))
            (:`then_1`
              (`self.Explode` :!label _label)))
          (else
            (goto _label)))))
    (:`then_2`
      (`self.DelayedDestroyProjectile`))))

(fn `OnBounce`
  (params (ImpactResultImpactPoint :type "Vector Structure") (ImpactResultHitComponent :type "PrimitiveComponent Object Reference"))
  (`self.Explode`)
  (`self.DelayedDestroyProjectile`))

(fn `RemoveFromOverlapped`
  (params (Vehicle :type "/Game/Blueprints/Player/MidVehicleBP/BP_BaseVehicle Object Reference"))
  (if (and (`KismetArrayLibrary.Array_Contains` (`self.OverlappedVehicles`) Vehicle) (not (`PrimitiveComponent.IsOverlappingActor` (`self.VehicleOverlap`) Vehicle)))
    (`KismetArrayLibrary.Array_RemoveItem` (`self.OverlappedVehicles`) Vehicle)))

(fn `UserConstructionScript`
  (`parent.UserConstructionScript`)
  (set `RadialForceComponent.DestructibleDamage` (`self.DMDamage`) (`self.WorldRadialForce`))
  (set `RadialForceComponent.ImpulseStrength` (`self.WorldImpactStrength`) (`self.WorldRadialForce`))
  (set `RadialForceComponent.ImpulseStrength` (`self.VehicleImpactStrength`) (`self.VehicleRadialForce`)))