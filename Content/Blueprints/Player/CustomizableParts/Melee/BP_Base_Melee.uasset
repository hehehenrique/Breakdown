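; Base Blueprint for a customizable melee weapon part on a vehicle, tracking which other vehicles are within its reach.
; MeleeRangeOverlap events resolve hit actors or their child-actor parents to BP_MidVehicleWithTurret, maintaining VehiclesInMeleeRange without the owning ParentVehicle.
; Removal waits until the vehicle no longer overlaps, and debug prints fire for the player's vehicle.
; No damage is applied here, and the construction script's SetupCollision is empty.
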(event `self.MeleeRangeOverlap.OnComponentBeginOverlap`
  (params (OverlappedComponent :type "PrimitiveComponent Object Reference") (OtherActor :type "Actor Object Reference") (OtherComp :type "PrimitiveComponent Object Reference") (OtherBodyIndex :type Integer) (bFromSweep :type Boolean) (SweepResult :type "HitResult Structure (by ref)"))
  (`self.OnBeginOverlap` OtherActor OtherComp))

(event `self.MeleeRangeOverlap.OnComponentEndOverlap`
  (params (OverlappedComponent :type "PrimitiveComponent Object Reference") (OtherActor :type "Actor Object Reference") (OtherComp :type "PrimitiveComponent Object Reference") (OtherBodyIndex :type Integer))
  (`self.OnEndOverlap` OtherActor OtherComp))

(fn `OnBeginOverlap`
  (params (OverlappedActor :type "Actor Object Reference") (OverlappedComponent :type "PrimitiveComponent Object Reference"))
  (locals (OverlappedVehicle :type "/Game/Blueprints/Player/MidVehicleBP/BP_MidVehicleWithTurret Object Reference"))
  (bind _vehiclesinmeleerange (`self.VehiclesInMeleeRange`))
  (bind _overlappedvehicle (`local.OverlappedVehicle`))
  (`|ExecutionSequence`
    (:`then_0`
      ;[1 1 1] Get Vehicle Reference
      (if (`self.IsChildActor` OverlappedActor)
        (bind _asbp_mid_vehicle_with_turret (cast `/Game/Blueprints/Player/MidVehicleBP/BP_MidVehicleWithTurret` (`self.GetParentActor` OverlappedActor)))
        (set `local.OverlappedVehicle` _asbp_mid_vehicle_with_turret)
        (else
          (bind _asbp_mid_vehicle_with_turret_2 (cast `/Game/Blueprints/Player/MidVehicleBP/BP_MidVehicleWithTurret` OverlappedActor))
          (set `local.OverlappedVehicle` _asbp_mid_vehicle_with_turret_2))))
    (:`then_1`
      ;[1 1 1] Add to actively damaged Vehicle array and start timer handle
      (if (!= (`local.OverlappedVehicle`) (`self.ParentVehicle`))
        (if (not (`KismetArrayLibrary.Array_Contains` _vehiclesinmeleerange (`local.OverlappedVehicle`)))
          (`KismetArrayLibrary.Array_AddUnique` _vehiclesinmeleerange _overlappedvehicle)
          (if (== (`self.ParentVehicle`) (`GameplayStatics.GetPlayerPawn` 0))
            (`KismetSystemLibrary.PrintString` (`KismetSystemLibrary.GetDisplayName` _overlappedvehicle) true true (struct :`R` 0.017054 :`G` 1.0 :`A` 1.0))))))))

(fn `OnEndOverlap`
  (params (OverlappedActor :type "Actor Object Reference") (OverlappedComponent :type "PrimitiveComponent Object Reference"))
  (locals (OverlappedVehicle :type "/Game/Blueprints/Player/MidVehicleBP/BP_MidVehicleWithTurret Object Reference"))
  (bind _vehiclesinmeleerange (`self.VehiclesInMeleeRange`))
  (`|ExecutionSequence`
    (:`then_0`
      (if (`self.IsChildActor` OverlappedActor)
        (bind _asbp_mid_vehicle_with_turret (cast `/Game/Blueprints/Player/MidVehicleBP/BP_MidVehicleWithTurret` (`self.GetParentActor` OverlappedActor)))
        (set `local.OverlappedVehicle` _asbp_mid_vehicle_with_turret)
        (else
          (bind _asbp_mid_vehicle_with_turret_2 (cast `/Game/Blueprints/Player/MidVehicleBP/BP_MidVehicleWithTurret` OverlappedActor))
          (set `local.OverlappedVehicle` _asbp_mid_vehicle_with_turret_2))))
    (:`then_1`
      (if (and (`KismetArrayLibrary.Array_Contains` _vehiclesinmeleerange (`local.OverlappedVehicle`)) (not (`PrimitiveComponent.IsOverlappingActor` (`self.MeleeRangeOverlap`) (`local.OverlappedVehicle`))))
        (`KismetArrayLibrary.Array_RemoveItem` _vehiclesinmeleerange (`local.OverlappedVehicle`))
        (if (== (`GameplayStatics.GetPlayerPawn` 0) (`self.ParentVehicle`))
          (`KismetSystemLibrary.PrintString` (`KismetStringLibrary.Concat_StrStr` "goodbye " (`KismetSystemLibrary.GetDisplayName` (`local.OverlappedVehicle`))) true true (struct :`R` 1.0 :`B` 0.123568 :`A` 1.0)))))))

(fn `SetupCollision`)

(fn `UserConstructionScript`
  (`self.SetupCollision`))