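; Base vehicle turret, a child actor of BP_MidVehicleWithTurret, that tracks the vehicle's aim target and fires projectiles.
; Each tick it rotates poseable-mesh bones with interpolated look-at rotations, splitting yaw and pitch between two joints.
; The cannon component attaches to a mesh socket at construction.
; ShootProjectile spawns ProjectileClass at the cannon, oriented toward the parent vehicle's separate ProjectileTarget.
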(event `self.ReceiveTick`
  (params (DeltaSeconds :type "Float (single-precision)"))
  (`self.AdjustTurretAngle`))

(fn `AdjustTurretAngle`
  (locals (OwnerTurretAimTarget :type "SphereComponent Object Reference"))
  (bind _turretposeablemesh (`self.TurretPoseableMesh`))
  (`|ExecutionSequence`
    (:`then_0`
      (bind _asbp_mid_vehicle_with_turret (cast `/Game/Blueprints/Player/MidVehicleBP/BP_MidVehicleWithTurret` (`self.GetParentActor`)))
      (set `local.OwnerTurretAimTarget` (`/Game/Blueprints/Player/MidVehicleBP/BP_MidVehicleWithTurret.TurretAimTarget` _asbp_mid_vehicle_with_turret)))
    (:`then_1`
      ;[1 1 1] Align Horizontal Piece
      (bind _returnvalue (`PoseableMeshComponent.GetBoneRotationByName` _turretposeablemesh "Weapon_JT_1" "WorldSpace"))
      (bind _returnvalue_2 (`PoseableMeshComponent.GetBoneLocationByName` _turretposeablemesh "Weapon_JT_2" "WorldSpace"))
      (bind _returnvalue_3 (`PoseableMeshComponent.GetBoneRotationByName` _turretposeablemesh "Weapon_JT_1" "ComponentSpace"))
      (bind _returnvalue_4 (`PoseableMeshComponent.GetBoneRotationByName` _turretposeablemesh "Weapon_JT_2" "ComponentSpace"))
      (bind (_returnvalue_roll _returnvalue_pitch) (`KismetMathLibrary.BreakRotator` (`KismetMathLibrary.FindLookAtRotation` _returnvalue_2 (`SceneComponent.K2_GetComponentLocation` (`local.OwnerTurretAimTarget`)))))
      (`PoseableMeshComponent.SetBoneRotationByName` _turretposeablemesh "Weapon_JT_2" (`KismetMathLibrary.RInterpTo` _returnvalue_4 (`KismetMathLibrary.MakeRotator` (.roll _returnvalue_3) (- _returnvalue_pitch (.pitch _returnvalue)) (.yaw _returnvalue_3)) (`GameplayStatics.GetWorldDeltaSeconds`) 20.0) "ComponentSpace"))
    (:`then_2`
      ;[1 1 1] Align Vertical Piece
      (bind _returnvalue_5 (`PoseableMeshComponent.GetBoneRotationByName` _turretposeablemesh "Weapon_Root" "WorldSpace"))
      (bind _returnvalue_6 (`PoseableMeshComponent.GetBoneLocationByName` _turretposeablemesh "Weapon_JT_1" "WorldSpace"))
      (bind _returnvalue_7 (`PoseableMeshComponent.GetBoneRotationByName` _turretposeablemesh "Weapon_JT_1" "ComponentSpace"))
      (bind (_returnvalue_roll_2 _returnvalue_pitch_2 _returnvalue_yaw) (`KismetMathLibrary.BreakRotator` (`KismetMathLibrary.FindLookAtRotation` _returnvalue_6 (`SceneComponent.K2_GetComponentLocation` (`local.OwnerTurretAimTarget`)))))
      (`PoseableMeshComponent.SetBoneRotationByName` _turretposeablemesh "Weapon_JT_1" (`KismetMathLibrary.RInterpTo` _returnvalue_7 (`KismetMathLibrary.MakeRotator` 0.0 0.0 (- _returnvalue_yaw (.yaw _returnvalue_5))) (`GameplayStatics.GetWorldDeltaSeconds`) 20.0) "ComponentSpace"))))

(fn `GetParentVehicle`
  (returns (ParentVehicle :type "/Game/Blueprints/Player/MidVehicleBP/BP_MidVehicleWithTurret Object Reference"))
  (bind _asbp_mid_vehicle_with_turret (cast `/Game/Blueprints/Player/MidVehicleBP/BP_MidVehicleWithTurret` (`self.GetParentActor`)))
  (return _asbp_mid_vehicle_with_turret))

(fn `ShootProjectile`
  (bind _returnvalue_location (`KismetMathLibrary.BreakTransform` (`SceneComponent.K2_GetComponentToWorld` (`self.TurretCannon`))))
  (`|SpawnActorFromClass` (`self.ProjectileClass`) (`KismetMathLibrary.MakeTransform` _returnvalue_location (`KismetMathLibrary.FindLookAtRotation` _returnvalue_location (`SceneComponent.K2_GetComponentLocation` (`/Game/Blueprints/Player/MidVehicleBP/BP_MidVehicleWithTurret.ProjectileTarget` (`self.GetParentVehicle`))))) "AdjustIfPossibleButAlwaysSpawn" "OverrideRootScale" self self self))

(fn `UserConstructionScript`
  (`SceneComponent.K2_AttachToComponent` (`self.TurretCannon`) (`self.TurretPoseableMesh`) "Weapon_JT_3" "KeepRelative" "KeepRelative" "KeepRelative" true))