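; Base class for customizable vehicle turrets, handling aiming, firing, ammo, reloads and overheating.
; The local player rotates poseable-mesh bones toward the vehicle's aim target and line-traces from the camera for the projectile target, sending bone rotations to the server.
; Shots spawn locally, then multicast for other machines to spawn their own, with recoil impulses and curve-driven spread that reverses after firing.
; Missile pickups replace normal fire; ultimate ammo suspends ammo use and heat updates.
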(event `UltimateAmmoActivated`
  (params (duration :type "Float (double-precision)" :default 1.0))
  (set `self.UltimateAmmoActive` true)
  (`KismetSystemLibrary.RetriggerableDelay` duration)
  (set `self.UltimateAmmoActive` false))

(event `SetBoneRotsServer`
  (params (HorizontalRot :type "Rotator Structure") (VerticalRot :type "Rotator Structure"))
  ;[1 1 1] Enforce Bone Rotation Vars Replication
  (set `self.HorizontalBoneRot` HorizontalRot)
  (set `self.VerticalBoneRot` VerticalRot))

(event `self.ReceiveTick`
  (params (DeltaSeconds :type "Float (single-precision)"))
  (bind _parentvehicle (`self.ParentVehicle`))
  (if (`Pawn.IsLocallyControlled` _parentvehicle)
    (if (`/Game/Blueprints/Player/MidVehicleBP/BP_BaseVehicle.isAlive` _parentvehicle)
      (`|ExecutionSequence`
        (:`then_0`
          (`self.AdjustTurretAngle`))
        (:`then_1`
          (`self.AdjustProjectileTargetLocation`))
        (:`then_2`
          (`self.UpdateJamProgress`))))
    (else
      (`self.ReplicateTurretPose`))))

(event `Reload`
  (if (and (!= (`self.CurrentAmmo`) (`self.MaxAmmo`)) (not (`self.isOverheated`)) (not (`self.isReloading`)) (not (`/Game/Blueprints/Player/MidVehicleBP/BP_BaseVehicle.MissileLauncherActive` (`self.ParentVehicle`))))
    (`self.StopShooting`)
    (set `self.isReloading` true)
    (`KismetSystemLibrary.Delay` (`self.ReloadTime`))
    (if (`self.isReloading`)
      (set `self.CurrentAmmo` (`self.MaxAmmo`))
      (set `self.isReloading` false)
      (set `self.canShoot` true)
      (if (`self.isTryingToShoot`)
        (`self.StartShooting`)))))

(event `Shoot`
  (params (Pressed :type Boolean))
  ;[1 1 1] Shooting
  (if Pressed
    (if (`/Game/Blueprints/Player/MidVehicleBP/BP_BaseVehicle.isAlive` (`self.ParentVehicle`))
      (`self.OnTriggerPress`))
    (else
      (`self.OnTriggerReleased`))))

(event `JustShot`
  (params (ProjectileTransform :type "Transform Structure"))
  ;[1 1 1] RateOfFire
  (`/Engine/EditorBlueprintResources/ActorMacros.Switch Has Authority`
    (:`Authority`
      (`self.ShootMulticast` ProjectileTransform))
    (:`Remote`
      (`self.ShootFromServer` ProjectileTransform)))
  (set `self.canShoot` false)
  (set `self.recentlyShot` true)
  (if (not (`/Game/Blueprints/Player/MidVehicleBP/BP_BaseVehicle.MissileLauncherActive` (`self.ParentVehicle`)))
    (if (not (`self.UltimateAmmoActive`))
      (`/Engine/EditorBlueprintResources/StandardMacros.DecrementInt` (`self.CurrentAmmo`)
        (:`  `
          _)))
    (`ActorComponent.SetActive` (`self.MuzzleFlash`) true true)
    (`self.ApplyRecoilForceOnVehicle`)
    (`self.PlayBulletShotSound`))
  (`KismetSystemLibrary.Delay` (`self.GetNextProjectileDelay`))
  (set `self.canShoot` true)
  (set `self.recentlyShot` false)
  (if (`self.isTryingToShoot`)
    (`self.ShootProjectile`)
    (else
      (`self.StoppedShooting`))))

(event `ShootFromServer`
  (params (ProjectileTransform :type "Transform Structure"))
  ;[1 1 1] RateOfFire
  (`self.ShootMulticast` ProjectileTransform))

(event `ShootMulticast`
  (params (ProjectileTransform :type "Transform Structure"))
  (bind _parentvehicle (`self.ParentVehicle`))
  (bind _parentvehicle_2 (`self.ParentVehicle`))
  (bind _parentvehicle_3 (`self.ParentVehicle`))
  (`self.PlayShootAnim`)
  (if (`Pawn.IsLocallyControlled` _parentvehicle_3)
    _
    (elif (`/Game/Blueprints/Player/MidVehicleBP/BP_BaseVehicle.MissileLauncherActive` _parentvehicle_3)
      (`|SpawnActorFromClass` "/Game/Blueprints/Projectiles/BP_Missile_Projectile.BP_Missile_Projectile_C" ProjectileTransform "Undefined" "OverrideRootScale" self _parentvehicle _parentvehicle)
      (else
        (`|SpawnActorFromClass` (`self.ProjectileClass`) ProjectileTransform "Undefined" "OverrideRootScale" self _parentvehicle_2 _parentvehicle_2)
        (`ActorComponent.SetActive` (`self.MuzzleFlash`) true true)
        (`self.ApplyRecoilForceOnVehicle`)
        (`self.PlayBulletShotSound`)))))

(event `OnTriggerPress`
  (`|ExecutionSequence`
    (:`then_1`
      (set `self.isTryingToShoot` true)
      (`self.StartShooting`))))

(event `OnTriggerReleased`
  (set `self.isTryingToShoot` false))

(event `OnGunOverheated`)

(event `StartShooting`
  (if (`self.GetShouldShoot`)
    (`|ExecutionSequence`
      (:`then_0`
        (`TimelineComponent.SetPlayRate` (`self.InaccuracyTimeline`) 1.0)
        (bind (_direction _inaccuracyovertime) (`Timeline|InaccuracyTimeline`)
          (:`Update`
            (set `self.CurrentInaccuracy` _inaccuracyovertime))))
      (:`then_2`
        (`self.ShootProjectile`)))
    (elif (`self.GetShouldReload`)
      (`self.Reload`))))

(event `StoppedShooting`
  (bind _inaccuracytimeline (`self.InaccuracyTimeline`))
  (bind (_mintime _maxtime) (`CurveBase.GetTimeRange` (`self.AccuracyCurve`)))
  (`|ExecutionSequence`
    (:`then_0`
      (if (< _maxtime (`TimelineComponent.GetPlaybackPosition` (`self.InaccuracyTimeline`)))
        (`TimelineComponent.SetNewTime` _inaccuracytimeline _maxtime) ; Makes it so the accuracy timeline will start reversing from the time value in which it reached maximum innaccuracy
      ))
    (:`then_1`
      (`TimelineComponent.SetPlayRate` _inaccuracytimeline _maxtime) ; Makes resetting the accuracy to initial only last 1 second
    )
    (:`then_2`
      (`TimelineComponent.Reverse` (`self.InaccuracyTimeline`)) ; Start reversing, minimizing spread
    )))

(event `ResetTurret`
  (set `self.JamProgress` 0.0)
  (set `self.isOverheated` false)
  (set `self.recentlyShot` false)
  (set `self.isTryingToShoot` false)
  (set `self.canShoot` true)
  (set `self.UltimateAmmoActive` false)
  (set `self.CurrentAmmo` (`self.MaxAmmo`))
  (set `self.isReloading` false))

(fn `AdjustProjectileTargetLocation`
  (bind _projectiletarget (`self.ProjectileTarget`))
  (bind _parentvehicle (`self.ParentVehicle`))
  (bind _camera (`/Game/Blueprints/Player/MidVehicleBP/BP_BaseVehicle.Camera` _parentvehicle))
  (bind _returnvalue (`SceneComponent.K2_GetComponentLocation` _camera))
  (bind _returnvalue_2 (`SceneComponent.GetForwardVector` _camera))
  (bind _returnvalue_3 (+ _returnvalue (* _returnvalue_2 (`KismetMathLibrary.VSize` (- (`SceneComponent.K2_GetComponentLocation` (`/Game/Blueprints/Player/MidVehicleBP/BP_BaseVehicle.SpringCameraScene` _parentvehicle)) _returnvalue)))))
  (bind _returnvalue_4 (+ _returnvalue_3 (* _returnvalue_2 10000.0)))
  (if (`Pawn.IsLocallyControlled` (`self.ParentVehicle`))
    (bind (_outhit _returnvalue_5) (`KismetSystemLibrary.LineTraceSingle` _returnvalue_3 _returnvalue_4 "TraceTypeQuery1" false (`|MakeArray` self (`self.ParentVehicle`) :!type "Actor Object Reference")))
    (if _returnvalue_5
      (`SceneComponent.K2_SetWorldLocation` _projectiletarget (`.ImpactPoint` (`GameplayStatics.BreakHitResult` _outhit)) false false)
      (else
        (`SceneComponent.K2_SetWorldLocation` _projectiletarget _returnvalue_4 false false)))))

(fn `AdjustTurretAngle`
  (locals (OwnerTurretAimTarget :type "SphereComponent Object Reference"))
  (bind _pm_turretbase (`self.PM_TurretBase`))
  (bind (_returnvalue_x _returnvalue_y _returnvalue_z) (`KismetMathLibrary.BreakVector` (`SceneComponent.GetUpVector` (`Actor.RootComponent` (`self.ParentVehicle`)))))
  (`|ExecutionSequence`
    (:`then_0`
      ;[1 1 1] Set Local Variable
      (set `local.OwnerTurretAimTarget` (`/Game/Blueprints/Player/MidVehicleBP/BP_BaseVehicle.TurretAimTarget` (`self.ParentVehicle`))))
    (:`then_1`
      ;[1 1 1] Align Horizontal Piece
      (bind _returnvalue (`PoseableMeshComponent.GetBoneRotationByName` _pm_turretbase (`self.WeaponRootSocketName`) "WorldSpace"))
      (bind _returnvalue_2 (`PoseableMeshComponent.GetBoneLocationByName` _pm_turretbase (`self.HorizontalJointName`) "WorldSpace"))
      (bind _returnvalue_3 (`PoseableMeshComponent.GetBoneRotationByName` _pm_turretbase (`self.HorizontalJointName`) "ComponentSpace"))
      (bind (_returnvalue_roll _returnvalue_pitch _returnvalue_yaw) (`KismetMathLibrary.BreakRotator` (`KismetMathLibrary.FindLookAtRotation` _returnvalue_2 (`SceneComponent.K2_GetComponentLocation` (`local.OwnerTurretAimTarget`)))))
      (bind _output_get (set `self.HorizontalBoneRot` (`KismetMathLibrary.RInterpTo` _returnvalue_3 (`KismetMathLibrary.MakeRotator` 0.0 0.0 (- _returnvalue_yaw (.yaw _returnvalue))) (`GameplayStatics.GetWorldDeltaSeconds`) (`self.TurretRotationSpeed`))))
      (`PoseableMeshComponent.SetBoneRotationByName` _pm_turretbase (`self.HorizontalJointName`) _output_get "ComponentSpace"))
    (:`then_2`
      ;[1 1 1] Align Vertical Piece
      (bind _returnvalue_4 (`PoseableMeshComponent.GetBoneRotationByName` _pm_turretbase (`self.HorizontalJointName`) "WorldSpace"))
      (bind _returnvalue_5 (`PoseableMeshComponent.GetBoneLocationByName` _pm_turretbase (`self.VerticalJointName`) "WorldSpace"))
      (bind _returnvalue_6 (`PoseableMeshComponent.GetBoneRotationByName` _pm_turretbase (`self.HorizontalJointName`) "ComponentSpace"))
      (bind _returnvalue_7 (`PoseableMeshComponent.GetBoneRotationByName` _pm_turretbase (`self.VerticalJointName`) "ComponentSpace"))
      (bind (_returnvalue_roll_2 _returnvalue_pitch_2) (`KismetMathLibrary.BreakRotator` (`KismetMathLibrary.FindLookAtRotation` _returnvalue_5 (`SceneComponent.K2_GetComponentLocation` (`local.OwnerTurretAimTarget`)))))
      (bind _output_get_2 (set `self.VerticalBoneRot` (`KismetMathLibrary.RInterpTo` _returnvalue_7 (`KismetMathLibrary.MakeRotator` (.roll _returnvalue_6) (`KismetMathLibrary.Lerp` 0.0 (- _returnvalue_pitch_2 (.pitch _returnvalue_4)) (`KismetMathLibrary.Abs` _returnvalue_z)) (.yaw _returnvalue_6)) (`GameplayStatics.GetWorldDeltaSeconds`) (`self.TurretRotationSpeed`))))
      (`PoseableMeshComponent.SetBoneRotationByName` _pm_turretbase (`self.VerticalJointName`) _output_get_2 "ComponentSpace"))
    (:`then_3`
      ;[1 1 1] Enforce Replication
      (`/Engine/EditorBlueprintResources/ActorMacros.Switch Has Authority`
        (:`Remote`
          (`self.SetBoneRotsServer` (`self.HorizontalBoneRot`) (`self.VerticalBoneRot`)))))))

(fn `ApplyRecoilForceOnVehicle`
  ;[1 1 1] Applies some recoil with the desired force on the parent vehicle
  (`PrimitiveComponent.AddImpulseAtLocation` (`/Game/Blueprints/Player/MidVehicleBP/BP_BaseVehicle.SM_Body` (`self.ParentVehicle`)) (* (`SceneComponent.GetForwardVector` (`self.TurretCannon`)) (* (`self.VehicleRecoilForce`) -1.0)) (`SceneComponent.K2_GetComponentLocation` (`self.TurretCannon`)) "None"))

(fn `GetNextProjectileDelay`
  (returns (DelayTime :type "Float (double-precision)"))
  (bind _parentvehicle (`self.ParentVehicle`))
  (if (`/Game/Blueprints/Player/MidVehicleBP/BP_BaseVehicle.MissileLauncherActive` _parentvehicle)
    (return (/ 1.0 (`.MissileLauncherRateOfFire_29_BA6256C34730CAAE9821ED849DBF1BB5` (break `/Game/Blueprints/PickUps/Data/PickUpInfo` (`/Game/Blueprints/Player/MidVehicleBP/BP_BaseVehicle.PickUpInfo` _parentvehicle)))))
    (else
      (return (/ 1.0 (`self.rateOfFire`))))))

(fn `GetPreciseProjectileTransform`
  (returns (ProjectileT :type "Transform Structure"))
  (bind _returnvalue (`SceneComponent.K2_GetComponentLocation` (`self.TurretCannon`)))
  (return (`KismetMathLibrary.MakeTransform` _returnvalue (`KismetMathLibrary.FindLookAtRotation` _returnvalue (`SceneComponent.K2_GetComponentLocation` (`self.ProjectileTarget`))))))

(fn `GetRandomProjectileTransform`
  (returns (ProjectileT :type "Transform Structure"))
  (bind _currentinaccuracy (`self.CurrentInaccuracy`))
  (bind _returnvalue (`SceneComponent.K2_GetComponentLocation` (`self.TurretCannon`)))
  (bind _returnvalue_2 (`KismetMathLibrary.FindLookAtRotation` _returnvalue (`SceneComponent.K2_GetComponentLocation` (`self.ProjectileTarget`))))
  (return (`KismetMathLibrary.MakeTransform` _returnvalue (`KismetMathLibrary.FindLookAtRotation` (`KismetMathLibrary.MakeVector` 0.0) (+ (* (`KismetMathLibrary.Normal` (+ (* (`KismetMathLibrary.GetUpVector` _returnvalue_2) (`KismetMathLibrary.RandomFloatInRange` -1.0 1.0)) (* (`KismetMathLibrary.GetRightVector` _returnvalue_2) (`KismetMathLibrary.RandomFloatInRange` -1.0 1.0)))) (* (`KismetMathLibrary.RandomFloatInRange` (* -1.0 _currentinaccuracy) _currentinaccuracy) 0.01)) (`KismetMathLibrary.Conv_RotatorToVector` _returnvalue_2))))))

(fn `GetShouldReload`
  (returns (shouldShoot :type Boolean))
  (return (and (`self.canShoot`) (== (`self.CurrentAmmo`) 0) (not (`self.isReloading`)) (`self.isTryingToShoot`))))

(fn `GetShouldShoot`
  (returns (shouldShoot :type Boolean))
  (return (and (`self.canShoot`) (or (and (< 0 (`self.CurrentAmmo`)) (not (`self.isReloading`)) (`self.isTryingToShoot`) (not (`self.isOverheated`))) (`/Game/Blueprints/Player/MidVehicleBP/BP_BaseVehicle.MissileLauncherActive` (`self.ParentVehicle`))))))

(fn `ParentVehicleNotified`
  (`parent.ParentVehicleNotified`)
  (`/Game/Blueprints/Player/MidVehicleBP/BP_BaseVehicle.FinishInitialiseVehicle` (`self.ParentVehicle`) self))

(fn `PlayBulletShotSound`
  (`GameplayStatics.PlaySoundAtLocation` (`|GetArrayItem` (`self.BulletShotSounds`) (`KismetMathLibrary.RandomIntegerInRange` 0 (- (`KismetArrayLibrary.Array_Length` (`self.BulletShotSounds`)) 1))) (`SceneComponent.K2_GetComponentLocation` (`self.TurretCannon`)) (struct) 1.0 1.0 0.0 null null null))

(fn `PlayShootAnim`
  ;[1 1 1] Override in each children
)

(fn `ReplicateTurretPose`
  (`PoseableMeshComponent.SetBoneRotationByName` (`self.PM_TurretBase`) (`self.HorizontalJointName`) (`self.HorizontalBoneRot`) "ComponentSpace")
  (`PoseableMeshComponent.SetBoneRotationByName` (`self.PM_TurretBase`) (`self.VerticalJointName`) (`self.VerticalBoneRot`) "ComponentSpace"))

(fn `ShootProjectile`
  (locals (ProjectileTransform :type "Transform Structure"))
  (if (`self.GetShouldShoot`)
    (if (`/Game/Blueprints/Player/MidVehicleBP/BP_BaseVehicle.MissileLauncherActive` (`self.ParentVehicle`))
      (bind _output_get (set `local.ProjectileTransform` (`self.GetPreciseProjectileTransform`)))
      (`|SpawnActorFromClass` "/Game/Blueprints/Projectiles/BP_Missile_Projectile.BP_Missile_Projectile_C" _output_get "AdjustIfPossibleButAlwaysSpawn" "OverrideRootScale" self (`self.ParentVehicle`) self)
      (else
        (bind _output_get_2 (set `local.ProjectileTransform` (`self.GetRandomProjectileTransform`)))
        (`|SpawnActorFromClass` (`self.ProjectileClass`) _output_get_2 "AdjustIfPossibleButAlwaysSpawn" "OverrideRootScale" self (`self.ParentVehicle`) self)))
    (`self.JustShot` (`local.ProjectileTransform`))
    (elif (`self.GetShouldReload`)
      (`self.Reload`)
      (else
        (`self.StoppedShooting`)))))

(fn `StopShooting`
  (`self.StoppedShooting`))

(fn `UpdateJamProgress`
  (locals (JamIncrement :type "Float (double-precision)"))
  (if (not (`self.UltimateAmmoActive`))
    (`|ExecutionSequence`
      (:`then_0`
        ;[1 1 1] Add or decrease?
        (if (`self.isOverheated`)
          (set `local.JamIncrement` (* (`self.CoolingPerSecond`) -1.0) :!label _label)
          (elif (and (`self.recentlyShot`) (`self.isTryingToShoot`))
            (set `local.JamIncrement` (`self.HeatingPerSecond`))
            (else
              (goto _label)))))
      (:`then_1`
        ;[1 1 1] Update value
        (set `self.JamProgress` (`KismetMathLibrary.FClamp` (+ (`self.JamProgress`) (* (`local.JamIncrement`) (`GameplayStatics.GetWorldDeltaSeconds`))) 0.0 100.0)))
      (:`then_2`
        ;[1 1 1] Check if bool needs changing
        (if (`self.isOverheated`)
          (if (== (`self.JamProgress`) 0.0)
            (set `self.isOverheated` false))
          (elif (== 100.0 (`self.JamProgress`))
            (set `self.isOverheated` true)
            (`self.OnGunOverheated`)))))))

(fn `UserConstructionScript`
  (`parent.UserConstructionScript`)
  (`|ExecutionSequence`
    (:`then_0`
      ;[1 1 1] This makes it so that both of these components rotate with the turret
      ;;[1 1 1] Attach shooting point to end of barrel socket
      (`SceneComponent.K2_AttachToComponent` (`self.TurretCannon`) (`self.PM_TurretBase`) (`self.CannonEndSocketName`) "KeepRelative" "KeepRelative" "KeepRelative" true)
      ;;[1 1 1] Attach the Zoom Point of this turret to its end of barrel socket
      (`SceneComponent.K2_AttachToComponent` (`self.CameraZoomPoint`) (`self.PM_TurretBase`) (`self.CannonEndSocketName`) "KeepRelative" "KeepRelative" "KeepRelative" true)
      (`TimelineComponent.SetFloatCurve` (`self.InaccuracyTimeline`) (`self.AccuracyCurve`) "InaccuracyOverTime") ; Apply custom accuracy curve
      (set `self.CurrentInaccuracy` (`CurveFloat.GetFloatValue` (`self.AccuracyCurve`) 0.0)) ; Initialize this value for UI (reticle) purposes
      (set `self.CurrentAmmo` (`self.MaxAmmo`)) ; Set current ammo to max
      ;[1 1 1] Calculate gun jam variables
      (set `self.CoolingPerSecond` (/ 100.0 (`self.TimeForGunCooling`))) ; How much progress gets decremented every second
      (set `self.HeatingPerSecond` (/ 100.0 (`self.TimeBeforeGunJams`))))
    (:`then_1`
      (`SceneComponent.K2_AttachToComponent` (`self.VerticalJoint`) (`self.PM_TurretBase`) (`self.VerticalJointName`) "SnapToTarget" "SnapToTarget" "KeepWorld" true)
      (`SceneComponent.K2_AttachToComponent` (`self.SM_CoreBody`) (`self.VerticalJoint`) "None" "KeepWorld" "KeepWorld" "KeepWorld" true))))