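; Big gun turret part for the player's customizable vehicle that rotates its poseable mesh toward the owning vehicle's aim target.
; AdjustTurretAngle gets TurretAimTarget from the parent BP_MidVehicleWithTurret, then pitches the vertical joint and yaws the horizontal joint toward it.
; Both bones are set in component space from world look-at angles, offset by horizontal joint pitch or mesh yaw and smoothed with RInterpTo.
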(fn `AdjustTurretAngle`
  (locals (OwnerTurretAimTarget :type "SphereComponent Object Reference"))
  (bind _turretposeablemesh (`self.TurretPoseableMesh`))
  (bind (_returnvalue_roll _returnvalue_pitch _returnvalue_yaw) (`KismetMathLibrary.BreakRotator` (`SceneComponent.K2_GetComponentRotation` (`self.TurretPoseableMesh`))))
  (`|ExecutionSequence`
    (:`then_0`
      (bind _asbp_mid_vehicle_with_turret (cast `/Game/Blueprints/Player/MidVehicleBP/BP_MidVehicleWithTurret` (`self.GetParentActor`)))
      (set `local.OwnerTurretAimTarget` (`/Game/Blueprints/Player/MidVehicleBP/BP_MidVehicleWithTurret.TurretAimTarget` _asbp_mid_vehicle_with_turret)))
    (:`then_1`
      ;[1 1 1] Align Vertical Piece
      (bind _returnvalue (`PoseableMeshComponent.GetBoneRotationByName` _turretposeablemesh (`self.HorizontalJointName`) "WorldSpace"))
      (bind _returnvalue_2 (`PoseableMeshComponent.GetBoneLocationByName` _turretposeablemesh (`self.VerticalJointName`) "WorldSpace"))
      (bind _returnvalue_3 (`PoseableMeshComponent.GetBoneRotationByName` _turretposeablemesh (`self.HorizontalJointName`) "ComponentSpace"))
      (bind _returnvalue_4 (`PoseableMeshComponent.GetBoneRotationByName` _turretposeablemesh (`self.VerticalJointName`) "ComponentSpace"))
      (bind (_returnvalue_roll_2 _returnvalue_pitch_2) (`KismetMathLibrary.BreakRotator` (`KismetMathLibrary.FindLookAtRotation` _returnvalue_2 (`SceneComponent.K2_GetComponentLocation` (`local.OwnerTurretAimTarget`)))))
      (`PoseableMeshComponent.SetBoneRotationByName` _turretposeablemesh (`self.VerticalJointName`) (`KismetMathLibrary.RInterpTo` _returnvalue_4 (`KismetMathLibrary.MakeRotator` (.roll _returnvalue_3) (- _returnvalue_pitch_2 (.pitch _returnvalue)) (.yaw _returnvalue_3)) (`GameplayStatics.GetWorldDeltaSeconds`) 20.0) "ComponentSpace"))
    (:`then_2`
      ;[1 1 1] Align Horizontal Piece
      (`PoseableMeshComponent.GetBoneRotationByName` _turretposeablemesh (`self.WeaponRootSocketName`) "WorldSpace")
      (bind _returnvalue_5 (`PoseableMeshComponent.GetBoneLocationByName` _turretposeablemesh (`self.HorizontalJointName`) "WorldSpace"))
      (bind _returnvalue_6 (`PoseableMeshComponent.GetBoneRotationByName` _turretposeablemesh (`self.HorizontalJointName`) "ComponentSpace"))
      (bind (_returnvalue_roll_3 _returnvalue_pitch_3 _returnvalue_yaw_2) (`KismetMathLibrary.BreakRotator` (`KismetMathLibrary.FindLookAtRotation` _returnvalue_5 (`SceneComponent.K2_GetComponentLocation` (`local.OwnerTurretAimTarget`)))))
      (`PoseableMeshComponent.SetBoneRotationByName` _turretposeablemesh (`self.HorizontalJointName`) (`KismetMathLibrary.RInterpTo` _returnvalue_6 (`KismetMathLibrary.MakeRotator` 0.0 0.0 (- _returnvalue_yaw_2 _returnvalue_yaw)) (`GameplayStatics.GetWorldDeltaSeconds`) 20.0) "ComponentSpace"))))

(fn `UserConstructionScript`
  (`parent.UserConstructionScript`))