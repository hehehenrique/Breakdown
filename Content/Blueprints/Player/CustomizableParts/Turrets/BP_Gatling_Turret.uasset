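; Gatling turret, a child of a parent turret Blueprint, whose barrel must spin up before it can fire.
; Trigger press plays a timeline that ramps barrel speed and starts shooting when it finishes forward; release clears the charged flag and reverses it to spin down.
; The shoot check requires that flag alongside the parent's conditions.
; Each tick rolls the barrel bone on a poseable mesh by the current speed.
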(event `self.ReceiveBeginPlay`
  ;[1 1 1] Set Barrel Starting Rotation Speed
  (`TimelineComponent.SetPlayRate` (`self.BarrelRotationTimeline`) (`self.gunChargeTime`)))

(event `self.ReceiveTick`
  (params (DeltaSeconds :type "Float (single-precision)"))
  (`parent.ReceiveTick` DeltaSeconds)
  (`self.RotateGunBarrel`))

(event `self.OnTriggerPress`
  (`parent.OnTriggerPress`)
  (bind (_direction _rotationspeed) (`Timeline|BarrelRotationTimeline` :!label _label)
    (:`Update`
      (set `self.barrelRotateSpeed` _rotationspeed))
    (:`Finished`
      (if (`|EnumEquality` _direction "Forward")
        (set `self.gunCharged` true)
        (`self.StartShooting`)))))

(event `self.OnTriggerReleased`
  (`parent.OnTriggerReleased`)
  (set `self.gunCharged` false)
  (goto _label :!via `Reverse`))

(fn `GetShouldShoot`
  (returns (shouldShoot :type Boolean))
  (return (and (`parent.GetShouldShoot`) (`self.gunCharged`))))

(fn `RotateGunBarrel`
  (bind _returnvalue (`PoseableMeshComponent.GetBoneRotationByName` (`self.TurretPoseableMesh`) (`self.BarrelRotationJoint`) "ComponentSpace"))
  (`PoseableMeshComponent.SetBoneRotationByName` (`self.TurretPoseableMesh`) (`self.BarrelRotationJoint`) (`KismetMathLibrary.MakeRotator` (+ (.roll _returnvalue) (* (`self.barrelRotateSpeed`) (`self.barrelMaxSpeed`) (`GameplayStatics.GetWorldDeltaSeconds`))) (.pitch _returnvalue) (.yaw _returnvalue)) "ComponentSpace"))

(fn `UserConstructionScript`
  (`parent.UserConstructionScript`))