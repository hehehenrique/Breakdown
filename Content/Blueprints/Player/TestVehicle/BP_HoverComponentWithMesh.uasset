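; A hover component for BP_ArcadeVehicleWithMesh that acts as a suspension point, pushing the vehicle up off the ground.
; Each tick it line traces along its negative up vector to the hover distance, ignoring the vehicle and drawing debug lines.
; On a hit, a spring-damper force from compression and its rate of change is applied to the vehicle's root primitive at the component's location.
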(event `self.ReceiveBeginPlay`
  ;[1 1 1] Casting to get the vehicle
  (bind _asbp_arcade_vehicle_with_mesh (cast `/Game/Blueprints/Player/TestVehicle/BP_ArcadeVehicleWithMesh` (`self.GetOwner`))
    (:`then`
      (set `self.ParentVehicle` _asbp_arcade_vehicle_with_mesh))
    (:`CastFailed`
      (`KismetSystemLibrary.PrintString` (`KismetStringLibrary.Concat_StrStr` "Could not find: " (`KismetStringLibrary.Conv_ObjectToString` _asbp_arcade_vehicle_with_mesh))))))

(event `self.ReceiveTick`
  (params (DeltaSeconds :type "Float (single-precision)"))
  (bind _returnvalue (`self.K2_GetComponentLocation`))
  ;[1 1 1] Checking for validity of parent vehicle
  (`/Engine/EditorBlueprintResources/StandardMacros.IsValid` (`self.ParentVehicle`)
    (:`Is Valid`
      ;[1 1 1] Starting line trace from vehicle location and towards it's up vector timed by the hover distance
      (bind (_outhit _returnvalue_2) (`KismetSystemLibrary.LineTraceSingle` _returnvalue (- _returnvalue (* (`self.GetUpVector`) (`self.HoverDistance`))) "TraceTypeQuery1" false (`|MakeArray` (`self.ParentVehicle`) :!type "Actor Object Reference") "ForOneFrame"))
      ;[1 1 1] Breaking hit result and getting the length of the line trace from start to where it hit the ground
      (bind _output_get (set `self.Hit` _returnvalue_2))
      (if _output_get
        (bind _output_get_2 (set `self.SpringCompression` (- (`self.HoverDistance`) (`.Distance` (`GameplayStatics.BreakHitResult` _outhit)))))
        ;[1 1 1] Adding force to the location of vehicle and saving the current spring compression as the last spring compression
        (`PrimitiveComponent.AddForceAtLocation` (cast `PrimitiveComponent` (`Actor.RootComponent` (`self.ParentVehicle`)) :!pure true) (* (`self.GetUpVector`) (+ (* (/ (- _output_get_2 (`self.PreviousSpringCompression`)) (`GameplayStatics.GetWorldDeltaSeconds`)) (`self.DampingCoefficient`)) (* _output_get_2 (`self.SpringCoefficient`)))) (`self.K2_GetComponentLocation`) "None")
        (set `self.PreviousSpringCompression` (`self.SpringCompression`))))
    (:`Is Not Valid`
      (`KismetSystemLibrary.PrintString` "Parent Vehicle is not valid" true true (struct :`G` 0.66 :`B` 1.0 :`A` 1.0) 0.01))))