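; Game mode that spawns each player in a turreted vehicle configured from that player's own settings.
; PostLogin increments the current player count and casts the new controller to PC_VehicleController, with no further live logic.
; The SpawnDefaultPawnAtTransform override spawns BP_MidVehicleWithTurret, passes in the controller's VehicleSettings at spawn, then possesses and returns it.
; Debug prints and a CustomSetup call remain disconnected.
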(event `self.K2_PostLogin`
  (params (NewPlayer :type "PlayerController Object Reference"))
  (`/Engine/EditorBlueprintResources/StandardMacros.IncrementInt` (`self.currentPlayers`)
    (:`  `
      (bind _aspc_vehicle_controller (cast `/Game/Game/PC_VehicleController` NewPlayer)))))

(fn `SpawnDefaultPawnAtTransform`
  (params (NewPlayer :type "Controller Object Reference") (SpawnTransform :type "Transform Structure (by ref)"))
  (returns (ReturnValue :type "Pawn Object Reference"))
  (bind _aspc_vehicle_controller (cast `/Game/Game/PC_VehicleController` NewPlayer))
  (bind _returnvalue (`|SpawnActorFromClass` "/Game/Blueprints/Player/MidVehicleBP/BP_MidVehicleWithTurret.BP_MidVehicleWithTurret_C" SpawnTransform "Undefined" "OverrideRootScale" NewPlayer (`/Game/Game/PC_VehicleController.VehicleSettings` _aspc_vehicle_controller) null))
  (`Controller.Possess` NewPlayer _returnvalue)
  (return _returnvalue))

(fn `UserConstructionScript`)