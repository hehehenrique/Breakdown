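; BP_PickUpPlatform is a pickup spawner that places a random pickup class from its list at its PickUpPoint.
; The first spawn follows an initial delay after BeginPlay.
; It binds to each spawned pickup's picked-up dispatcher, and a recharge event spawns a new random pickup after a respawn delay.
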(event `self.ReceiveBeginPlay`
  (`KismetSystemLibrary.Delay` (`self.InitialSpawnTime`))
  (`self.SpawnPickUp`))

(event `BeginRecharge`
  (`KismetSystemLibrary.Delay` (`self.RespawnDelay`))
  (`self.SpawnPickUp`))

(event `SpawnPickUp`
  (bind _pickupclasses (`self.PickUpClasses`))
  (bind _returnvalue (`|SpawnActorFromClass` (`|GetArrayItem` _pickupclasses (`KismetMathLibrary.RandomInteger` (`KismetArrayLibrary.Array_Length` _pickupclasses))) (`SceneComponent.K2_GetComponentToWorld` (`self.PickUpPoint`)) "AlwaysSpawn" "OverrideRootScale" null true null))
  (add `/Game/Blueprints/PickUps/BP_Base_PickUp.PickedUpDispatcher` _returnvalue (`|CreateDelegate` :!event `BeginRecharge`)))

(fn `UserConstructionScript`)